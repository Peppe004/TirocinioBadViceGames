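; Cleaning tool object that hosts a cleaning component and exposes a transform for attaching to the player.
; On BeginPlay it initializes BPCleaningComp with its collider and max filth amount, then disables that component's collision.
; Functions toggle static mesh collision between query-only and off, return the attach arrow transform, and report a fixed cleaning type.
; Interact is a stub, and the tool-type matching logic is left unconnected.
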(event OnComponentBeginOverlap(CleaningCompCollider)
  (params (OverlappedComponent :type Primitive%20Component%20Object%20Reference) (OtherActor :type Actor%20Object%20Reference) (OtherComp :type Primitive%20Component%20Object%20Reference) (OtherBodyIndex :type Integer) (bFromSweep :type Boolean) (SweepResult :type Hit%20Result%20Structure%20%28by%20ref%29)))

(event EventBeginPlay
  (bind _bp_cleaningcomp (Variables|Default|GetBP_CleaningComp))
  (|CallParentFunction)
  (Default|Initialize _bp_cleaningcomp (Variables|Default|GetCleaningCompCollider) (Variables|Default|GetMaxFilthAmount))
  (Default|DisableCollision _bp_cleaningcomp))

(event Collision|EventActorBeginOverlap
  (params (OtherActor :type Actor%20Object%20Reference))
  (|CallParentFunction OtherActor) ; This node is disabled and will not be called.\nDrag off pins to build functionality.
)

(event EventTick
  (params (DeltaSeconds :type Float%20%28single-precision%29))
  (|CallParentFunction DeltaSeconds) ; This node is disabled and will not be called.\nDrag off pins to build functionality.
)

(fn ConstructionScript
  (|CallParentFunction))

(fn DisableCollision
  (Collision|SetCollisionEnabled (Variables|Default|GetStaticMesh) "NoCollision")
  (return false))

(fn Interact
  (return false))

(fn EnableCollision
  (Collision|SetCollisionEnabled (Variables|Default|GetStaticMesh) "QueryOnly")
  (return false))

(fn ReturnArrowTransform
  (return (Transformation|GetWorldTransform (Variables|Default|GetAttachToPlayerArrow))))

(fn ReturnCleaningType
  (return "NewEnumerator0"))