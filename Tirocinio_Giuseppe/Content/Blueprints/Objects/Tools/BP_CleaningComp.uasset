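; Cleaning tool component that tracks how much filth a tool such as the mop holds.
; Adding filth subtracts stain hit points until the limit, then enlarges stains and signals a fully dirty mop; washing removes one filth unit.
; SpawnStain sphere-traces below the collider, spawns a surface-aligned blood stain and notifies the game instance.
; Interface functions toggle collider collision and report tool type; the rest are stubs.
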(event EventBeginPlay
  (Utilities|Casting|CastToBP_MainGameInstance (Game|GetGameInstance)))

(event EventCleanMop
  ;[0.15 0.15 0.15 0.5] MOP BEHAVIOR
  (if (== (Variables|Cleaning|GetFilth%20Amount%20) 0)
    (Development|PrintString "Mop already clean")
    (else
      (Variables|Cleaning|SetFilth%20Amount%20 (- (Variables|Cleaning|GetFilth%20Amount%20) 1))
      (Variables|Cleaning|SetIs%20Fully%20DIrty%20 false)
      (Development|PrintString "Washing mop"))))

(event EventAddFilthtoTool
  (params (HitActor :type Actor%20Object%20Reference))
  ;[0.15 0.15 0.15 0.5] MOP BEHAVIOR
  (if (< (Variables|Cleaning|GetFilth%20Amount%20) (Variables|Cleaning|GetMax%20Filth%20Amount))
    (Math|Integer|IncrementInt (Variables|Cleaning|GetFilth%20Amount%20)
      (:%20%20
        (Class|BPICleanableObject|SubtractHitPoints(Message) HitActor)))
    (else
      (Variables|Cleaning|SetFilth%20Amount%20 (Variables|Cleaning|GetMax%20Filth%20Amount))
      (Class|BPICleanableObject|MakeStainBigger(Message) HitActor)
      (Variables|Cleaning|SetIs%20Fully%20DIrty%20 true)
      (Default|CallOnMopFullyDirty))))

(fn Initialize
  (params (Collider :type Box%20Component%20Object%20Reference) (MaxFilthAmount :type Integer))
  (Variables|Default|SetCollider Collider)
  (Variables|Cleaning|SetMax%20Filth%20Amount MaxFilthAmount))

(fn SpawnStain
  (bind _collider (Variables|Default|GetCollider))
  (bind _returnvalue (Transformation|GetWorldLocation _collider))
  (bind _outhit (Collision|SphereTraceByChannel _returnvalue (+ _returnvalue (* (Math|Vector|GetUpVector _collider) -200)) 5.0 "TraceTypeQuery1" false 0 "ForDuration" true "(R=1.000000,G=0.000000,B=0.000000,A=1.000000)" "(R=0.000000,G=1.000000,B=0.000000,A=1.000000)" 2e+01))
  (Game|SpawnActorfromClass "/Game/Blueprints/Objects/CleanableObjects/BP_BloodStain.BP_BloodStain_C" (Math|Transform|MakeTransform (.Location (Collision|BreakHitResult _outhit)) (Math|Conversions|RotationFromXVector (.Normal (Collision|BreakHitResult _outhit))) "1.000000,1.000000,1.000000") "Undefined" "MultiplyWithRoot" 0 0)
  (bind _asbp_main_game_instance (Utilities|Casting|CastToBP_MainGameInstance (Game|GetGameInstance)))
  (Default|OnSpawnStain _asbp_main_game_instance))

(fn CheckBinCapacity
  (return false))

(fn DisableCollision
  (Collision|SetCollisionEnabled (Variables|Default|GetCollider) "NoCollision")
  (return false))

(fn EnableCollision
  (Collision|SetCollisionEnabled (Variables|Default|GetCollider) "QueryOnly")
  (return false))

(fn GetIsOpen
  (return false))

(fn GetMesh
  (return 0))

(fn GetQuestID
  (return "None"))

(fn Interact
  (return false))

(fn ReturnArrowTransform
  (return ""))

(fn ReturnBinCapacity
  (return 0))

(fn ReturnCleaningType
  (return (Variables|Cleaning|GetTool%20Type%20)))

(fn ReturnTrashInitiaLocation
  (return "0, 0, 0"))

(fn ReturnTrashTravelTransform
  (return ""))

(fn StartDialog
  (return false))

(fn UnlockDoor
  (return false))