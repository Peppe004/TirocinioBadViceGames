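; Interactable water bucket tool that washes the mop the player is holding.
; Interact takes the "Mop"-tagged held object from the player, sends it a clean message and dips it below the cleaning point with a timeline, then returns it.
; Player and mop communicate through message calls, and a CanWashMop flag with a short cooldown gates repeats.
; A glow timeline drives the lighting component's emissive highlight until washing stops it.
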(event Custom|MoveMopUpAndDown
  (if (Variables|Default|GetCan%20Wash%20Mop)
    (Variables|Default|SetCan%20Wash%20Mop false)
    (Class|BPIPlayer|ReleaseMop(Message) (Game|GetPlayerCharacter 0))
    (Variables|Default|SetStart%20Location (Transformation|GetWorldLocation (Variables|Default|GetCleaningMopPoint)))
    (Variables|Default|SetEnd%20Location (+ (Transformation|GetWorldLocation (Variables|Default|GetCleaningMopPoint)) (* (Math|Vector|VectorDown) 20)))
    (bind _held_object (Class|BPIPlayer|ReturnCurrentHeldObject(Message) (Game|GetPlayerCharacter 0)))
    (if (Actor|ActorHasTag _held_object "Mop")
      (Variables|Default|SetMop _held_object)
      (Utilities|FlowControl|Delay 0.2)
      (Class|BPIInterarct|CleanMop(Message) (Variables|Default|GetMop))
      (CallFunction|StopGlowing)
      (bind _alpha (Timeline|MoveMop PlayFromStart)
        (:Update
          (Transformation|SetActorLocation (Variables|Default|GetMop) (Math|Vector|Lerp(Vector) (Variables|Default|GetStart%20Location) (Variables|Default|GetEnd%20Location) _alpha) false false))
        (:Finished
          (CallFunction|ReturnMoptoPlayer))))))

(event Custom|ReturnMopToPlayer
  (Transformation|DetachFromActor (Variables|Default|GetMop) "KeepWorld" "KeepWorld" "KeepWorld")
  (Class|BPIPlayer|RetakeMop(Message) (Game|GetPlayerCharacter 0))
  (Variables|Default|SetMop 0)
  (Utilities|FlowControl|Delay 2.0)
  (Variables|Default|SetCan%20Wash%20Mop true))

(event EventBeginPlay
  (|CallParentFunction) ; This node is disabled and will not be called.\nDrag off pins to build functionality.
)

(event Collision|EventActorBeginOverlap
  (params (OtherActor :type Actor%20Object%20Reference))
  (|CallParentFunction OtherActor) ; This node is disabled and will not be called.\nDrag off pins to build functionality.
)

(event EventGlow
  ;[0.15 0.15 0.15 0.5] Inizia a lampeggiare
  (Components|Timeline|SetPlayRate (Variables|Default|GetGlowTimeline) (/ 2.0 2.5))
  (bind _alpha (Timeline|GlowTimeline PlayFromStart)
    (:Update
      (Default|SetValues (Variables|Default|GetBP_LightingComponent) (Math|Float|Lerp (Variables|Default|GetStartEmissive) (Variables|Default|GetEndEmissive) _alpha)))))

(event EventStopGlowing
  ;[0.15 0.15 0.15 0.5] Smette di lampeggiare
  (Audio|Components|Audio|Stop (Variables|Default|GetGlowTimeline))
  (Variables|Default|SetEndEmissive 0.0)
  (Default|SetValues (Variables|Default|GetBP_LightingComponent) 0.0))

(event EventSetCanWashMop
  (Variables|Default|SetCan%20Wash%20Mop true))

(fn ConstructionScript
  (|CallParentFunction))

(fn Interact
  (CallFunction|MoveMopUpandDown)
  (return false))