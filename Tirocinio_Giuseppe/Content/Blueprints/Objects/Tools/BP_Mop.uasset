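; Mop tool actor that the player can pick up and swing to clean matching dirty objects.
; Interacting triggers a timeline that rotates the mesh toward an arrow's rotation, with event tracks toggling the cleaning component's collision during the swing.
; Collider overlaps add filth to the mop from type-matched targets, or spawn a stain on floors when the mop is fully dirty.
; A second timeline drives the lighting component's emissive glow.
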(event OnComponentBeginOverlap(CleaningCompCollider)
  (params (OverlappedComponent :type Primitive%20Component%20Object%20Reference) (OtherActor :type Actor%20Object%20Reference) (OtherComp :type Primitive%20Component%20Object%20Reference) (OtherBodyIndex :type Integer) (bFromSweep :type Boolean) (SweepResult :type Hit%20Result%20Structure%20%28by%20ref%29))
  ;[0.15 0.15 0.15 0.5] CLEANING LOGIC
  (bind _output_get (Variables|/Game/Blueprints/Objects/Tools/BP_CleaningComp.BP_CleaningComp_C|SetHit%20Actor (Variables|Default|GetBP_CleaningComp) OtherActor))
  (if (Actor|ActorHasTag _output_get "Floor")
    (if (Variables|/Game/Blueprints/Objects/Tools/BP_CleaningComp.BP_CleaningComp_C|GetIs%20Fully%20DIrty%20 (Variables|Default|GetBP_CleaningComp))
      (Default|SpawnStain (Variables|Default|GetBP_CleaningComp)))
    (else
      (bind _matches_enum (Class|BPICleanableObject|MatchesEnum(Message) _output_get self))
      (if _matches_enum
        (Class|BPIInterarct|AddFilthtoTool(Message) (Variables|Default|GetBP_CleaningComp) _output_get)))))

(event EventBeginPlay
  (|CallParentFunction))

(event Collision|EventActorBeginOverlap
  (params (OtherActor :type Actor%20Object%20Reference))
  (|CallParentFunction OtherActor) ; This node is disabled and will not be called.\nDrag off pins to build functionality.
)

(event EventTick
  (params (DeltaSeconds :type Float%20%28single-precision%29))
  (|CallParentFunction DeltaSeconds))

(event EventDisableCleaningCompCollision
  ;[0.15 0.15 0.15 0.5] CLEANING LOGIC
  (Class|BPIInterarct|DisableCollision(Message) (Variables|Default|GetBP_CleaningComp)))

(event EventMoveTool
  ;[0.15 0.15 0.15 0.5] MOVE MOP
  (if (Variables|Default|GetCanMove)
    (Variables|Default|SetStartRotation (Variables|/Script/Engine.SceneComponent|GetRelativeRotation (Variables|Default|GetStaticMesh)))
    (Variables|Default|SetEndRotation (Variables|/Script/Engine.SceneComponent|GetRelativeRotation (Variables|Default|GetCleaningArrow)))
    (Variables|Default|SetCanMove false)
    (bind _alpha (Timeline|RotateTool PlayFromStart)
      (:Update
        (Transformation|SetRelativeRotation (Variables|Default|GetStaticMesh) (Math|Rotator|Lerp(Rotator) (Variables|Default|GetStartRotation) (Variables|Default|GetEndRotation) _alpha) false false))
      (:Finished
        (Variables|Default|SetCanMove true))
      (:EnableCollision
        (Default|EnableCollision (Variables|Default|GetBP_CleaningComp)))
      (:DisableCollision
        (Default|DisableCollision (Variables|Default|GetBP_CleaningComp))))))

(event EventCleanMop
  ;[0.15 0.15 0.15 0.5] CLEANING LOGIC
  (Default|CleanMop (Variables|Default|GetBP_CleaningComp)))

(event EventStopGlowing
  ;[0.15 0.15 0.15 0.5] smette di lampeggiare
  (Audio|Components|Audio|Stop (Variables|Default|GetToggleObjectLightTimeline))
  (Variables|Default|SetEndEmissive 0.0)
  (Default|SetValues (Variables|Default|GetBP_LightingComponent) 0.0))

(event EventGlow
  ;[0.15 0.15 0.15 0.5] Inizia a lampeggiare
  (Components|Timeline|SetPlayRate (Variables|Default|GetToggleObjectLightTimeline) (/ 2.0 2.5))
  (bind _alpha (Timeline|ToggleObjectLightTimeline PlayFromStart)
    (:Update
      (Default|SetValues (Variables|Default|GetBP_LightingComponent) (Math|Float|Lerp (Variables|Default|GetStartEmissive) (Variables|Default|GetEndEmissive) _alpha)))))

(event EventSetCanbePicked
  (Variables|Default|SetCanBePicked true))

(fn ConstructionScript
  (|CallParentFunction))

(fn DisableCollision
  (return false))

(fn EnableCollision
  (return false))

(fn ReturnArrowTransform
  (return (Transformation|GetRelativeTransform (Variables|Default|GetAttachToPlayerArrow))))

(fn Interact
  (Development|PrintString "Now Started Cleaning...")
  (Class|BPIInterarct|MoveTool(Message) self)
  (return false))

(fn ReturnCleaningType
  (return "NewEnumerator0"))

(fn GetCanbePicked
  (return (Variables|Default|GetCanBePicked)))