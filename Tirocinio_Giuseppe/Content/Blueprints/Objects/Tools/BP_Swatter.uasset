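; BP_Swatter is a pickable cleaning tool that plays a swing when used and removes hit points from targets it strikes.
; Interact runs a timeline that rotates the mesh toward a cleaning arrow, blocks re-triggering until finished, and toggles the cleaning component's collision during the swing.
; Overlapped actors lose hit points only when their enum check matches the swatter.
; A separate timeline drives an emissive glow through a lighting component.
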(event OnComponentBeginOverlap(CleaningCompCollider)
  (params (OverlappedComponent :type Primitive%20Component%20Object%20Reference) (OtherActor :type Actor%20Object%20Reference) (OtherComp :type Primitive%20Component%20Object%20Reference) (OtherBodyIndex :type Integer) (bFromSweep :type Boolean) (SweepResult :type Hit%20Result%20Structure%20%28by%20ref%29))
  ;[0.15 0.15 0.15 0.5] COLLISION DETECTION
  (bind _output_get (Variables|/Game/Blueprints/Objects/Tools/BP_CleaningComp.BP_CleaningComp_C|SetHit%20Actor (Variables|Default|GetBP_CleaningComp) OtherActor))
  (bind _matches_enum (Class|BPICleanableObject|MatchesEnum(Message) _output_get self))
  (if _matches_enum
    (Class|BPICleanableObject|SubtractHitPoints(Message) _output_get)))

(event EventMoveTool
  ;[0.15 0.15 0.15 0.5] TOOL MOVEMENT LOGIC
  (if (Variables|Default|GetCan%20Move)
    (Variables|Default|SetStart%20Rotation (Variables|/Script/Engine.SceneComponent|GetRelativeRotation (Variables|Default|GetStaticMesh)))
    (Variables|Default|SetEnd%20Rotation (Variables|/Script/Engine.SceneComponent|GetRelativeRotation (Variables|Default|GetCleaningArrow)))
    (Variables|Default|SetCan%20Move false)
    (bind _alpha (Timeline|Timeline PlayFromStart)
      (:Update
        (Transformation|SetRelativeRotation (Variables|Default|GetStaticMesh) (Math|Rotator|Lerp(Rotator) (Variables|Default|GetStart%20Rotation) (Variables|Default|GetEnd%20Rotation) _alpha) false false))
      (:Finished
        (Variables|Default|SetCan%20Move true))
      (:EnableCollision
        (Default|EnableCollision (Variables|Default|GetBP_CleaningComp)))
      (:DisableCollision
        (Default|DisableCollision (Variables|Default|GetBP_CleaningComp))))))

(event EventSetCanbePicked
  (Variables|Default|SetCanBePicked true))

(event EventGlow
  ;[0.15 0.15 0.15 0.5] Si illumina
  (Components|Timeline|SetPlayRate (Variables|Default|GetGlowTimeLine) (/ 2.0 2.5))
  (bind _alpha (Timeline|GlowTimeLine PlayFromStart)
    (:Update
      (Default|SetValues (Variables|Default|GetBP_LightingComponent) (Math|Float|Lerp (Variables|Default|GetStartEmissive) (Variables|Default|GetEndEmissive) _alpha)))))

(event EventStopGlowing
  ;[0.15 0.15 0.15 0.5] Smette di brillare
  (Audio|Components|Audio|Stop (Variables|Default|GetGlowTimeLine))
  (Variables|Default|SetEndEmissive 0.0)
  (Default|SetValues (Variables|Default|GetBP_LightingComponent) 0.0))

(fn ConstructionScript
  (|CallParentFunction))

(fn ReturnArrowTransform
  (return (Transformation|GetRelativeTransform (Variables|Default|GetAttachToPlayerArrow))))

(fn Interact
  (Development|PrintString "Using Swatter")
  (Default|MoveTool self)
  (return false))

(fn ReturnCleaningType
  (return (Variables|/Game/Blueprints/Objects/Tools/BP_CleaningComp.BP_CleaningComp_C|GetTool%20Type%20 (Variables|Default|GetBP_CleaningComp))))

(fn GetCanbePicked
  (return (Variables|Default|GetCanBePicked)))