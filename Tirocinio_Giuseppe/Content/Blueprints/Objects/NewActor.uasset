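; NewActor is a placeholder actor Blueprint with no working behavior.
; Its stub functions, which look like interface implementations, cover interaction, dialog, quests, doors, collision toggling and trash-bin cleaning, and return only default or empty values.
; BeginPlay, overlap and Tick events are disabled, and the construction script is empty.
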(event EventBeginPlay)

(event Collision|EventActorBeginOverlap
  (params (OtherActor :type Actor%20Object%20Reference)))

(event EventTick
  (params (DeltaSeconds :type Float%20%28single-precision%29)))

(fn ConstructionScript)

(fn CheckBinCapacity
  (return false))

(fn DisableCollision
  (return false))

(fn EnableCollision
  (return false))

(fn GetIsOpen
  (return false))

(fn GetMesh
  (return 0))

(fn GetQuestID
  (return "None"))

(fn Interact
  (return false))

(fn ReturnArrowTransform
  (return ""))

(fn ReturnBinCapacity
  (return 0))

(fn ReturnCleaningType
  (return "NewEnumerator0"))

(fn ReturnTrashInitiaLocation
  (return "0, 0, 0"))

(fn ReturnTrashTravelTransform
  (return ""))

(fn StartDialog
  (return false))

(fn UnlockDoor
  (return false))