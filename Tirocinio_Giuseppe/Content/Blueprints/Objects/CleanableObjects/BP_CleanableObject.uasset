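; BP_CleanableObject is a cleanable object with a cleaning type, hit points and a Stain child actor.
; Construction sizes its box from Size and hides the static mesh with collision off, while MatchesEnum compares a tool's cleaning type to its own.
; SubtractHitPoints tells the stain to clean, then at zero fires OnObjectCleaned and destroys the actor.
; Destruction notifies BP_MainGameInstance to update the cleaned-object objective.
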(event EventBeginPlay
  ;[0.15 0.15 0.15 0.5] BEGIN PLAY
  (|CallParentFunction))

(event Collision|EventActorBeginOverlap
  (params (OtherActor :type Actor%20Object%20Reference))
  (|CallParentFunction OtherActor) ; Questo nodo è disabilitato e non verrà chiamato.\nTrascina i pin per creare funzionalità.
)

(event EventTick
  (params (DeltaSeconds :type Float%20%28single-precision%29))
  (|CallParentFunction DeltaSeconds) ; Questo nodo è disabilitato e non verrà chiamato.\nTrascina i pin per creare funzionalità.
)

(event EventDestroyed
  ;[0.15 0.15 0.15 0.5] DESTRUCTION LOGIC
  (bind _asbp_main_game_instance (Utilities|Casting|CastToBP_MainGameInstance (Game|GetGameInstance)))
  (Default|CleanedObjectUpdate _asbp_main_game_instance)
  (Development|PrintString "Objective list has been updated..."))

(fn ConstructionScript
  (|CallParentFunction)
  (Components|Box|SetBoxExtent (Variables|Default|GetBox) (Variables|Default|GetSize) true)
  (Rendering|SetVisibility (Variables|Default|GetStaticMesh) false true)
  (Collision|SetCollisionEnabled (Variables|Default|GetStaticMesh) "NoCollision"))

(fn ReturnCleaningType
  (return (Variables|Default|GetType)))

(fn Interact
  (return false))

(fn MatchesEnum
  (params (Tool :type Actor%20Object%20Reference))
  (bind _newparam (Class|BPIInterarct|ReturnCleaningType(Message) Tool))
  (return (== (Math|Byte|MakeLiteralByte _newparam) (Math|Byte|MakeLiteralByte (Variables|Default|GetType)))))

(fn SubtractHitPoints
  ;[0.15 0.15 0.15 0.5] CLEANING LOGIC
  (Class|BPIDecal|CleanStain(Message) (Variables|/Script/Engine.ChildActorComponent|GetChildActor (Variables|Default|GetStain)))
  (bind _output_get (Variables|Default|SetHit%20Points (- (Variables|Default|GetHit%20Points) 1)))
  (if (== _output_get 0)
    (Default|CallOnObjectCleaned)
    (Actor|DestroyActor)
    (else
      (return false))))