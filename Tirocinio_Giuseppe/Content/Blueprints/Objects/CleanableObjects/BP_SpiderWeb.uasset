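; BP_SpiderWeb is a cleanable spider web object that feeds the game's web cleaning objective.
; On BeginPlay it increments the total webs-to-clean counter in BP_MainGameInstance, so each spawned web registers itself.
; When destroyed, it calls the game instance's cleaned webs update and prints a debug message.
; ReturnCleaningType reports a fixed enum value identifying its cleaning type.
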(event EventBeginPlay
  ;[0.15 0.15 0.15 0.5] INCRMEENTS SPECIFIC COUNTER IN THE GAMEINSTANCE
  (|CallParentFunction)
  (bind _asbp_main_game_instance (Utilities|Casting|CastToBP_MainGameInstance (Game|GetGameInstance)))
  (Math|Integer|IncrementInt (Variables|/Game/Blueprints/Singletons/BP_MainGameInstance.BP_MainGameInstance_C|GetTotalWebsToClean _asbp_main_game_instance)))

(event Collision|EventActorBeginOverlap
  (params (OtherActor :type Actor%20Object%20Reference))
  (|CallParentFunction OtherActor) ; This node is disabled and will not be called.\nDrag off pins to build functionality.
)

(event EventTick
  (params (DeltaSeconds :type Float%20%28single-precision%29))
  (|CallParentFunction DeltaSeconds) ; This node is disabled and will not be called.\nDrag off pins to build functionality.
)

(event EventDestroyed
  ;[0.15 0.15 0.15 0.5] DESTRUCTION LOGIC
  (bind _asbp_main_game_instance (Utilities|Casting|CastToBP_MainGameInstance (Game|GetGameInstance)))
  (Default|CleanedWebsUpdate _asbp_main_game_instance)
  (Development|PrintString "Objective list has been updated..."))

(fn ConstructionScript
  (|CallParentFunction))

(fn ReturnCleaningType
  (return "NewEnumerator1"))