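; BP_BloodStain is a cleanable blood stain object that grows when mopped with a dirty mop.
; Its MakeStainBigger event prints a debug message, then, while below MaxHitPoints, raises HitPoints and tells the Stain child actor to enlarge via MakeStainBiggerMessage.
; The construction script runs the parent's logic and sizes the Box component from BoxSize.
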(event EventBeginPlay
  (|CallParentFunction))

(event Collision|EventActorBeginOverlap
  (params (OtherActor :type Actor%20Object%20Reference))
  (|CallParentFunction OtherActor) ; This node is disabled and will not be called.\nDrag off pins to build functionality.
)

(event EventTick
  (params (DeltaSeconds :type Float%20%28single-precision%29))
  (|CallParentFunction DeltaSeconds) ; This node is disabled and will not be called.\nDrag off pins to build functionality.
)

(event EventMakeStainBigger
  (Development|PrintString "Mop is dirty, making stain bigger")
  (if (< (Variables|Default|GetHit%20Points) (Variables|Default|GetMaxHitPoints))
    (Math|Integer|IncrementInt (Variables|Default|GetHit%20Points)
      (:%20%20
        (Class|BPIDecal|MakeStainBigger(Message) (Variables|/Script/Engine.ChildActorComponent|GetChildActor (Variables|Default|GetStain)))))))

(fn ConstructionScript
  (|CallParentFunction)
  (Components|Box|SetBoxExtent (Variables|Default|GetBox) (Variables|Default|GetBoxSize) true))