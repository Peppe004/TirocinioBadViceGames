(event EventBeginPlay)

(event EventTick
  (params (DeltaSeconds :type Float%20%28single-precision%29)))

(fn ConstructionScript)

(fn CanCloseDoor
  (for _array_element (Collision|GetOverlappingActors (Variables|Default|GetBox) 0 :!class /Script/Engine.PrimitiveComponent)
    (if (or (Actor|ActorHasTag _array_element "Cart") (Actor|ActorHasTag _array_element "Player"))
      (bind _output_get (LocalVariables|SetCanCloseRoomDoor false))
      (return _output_get)))
  (return _output_get))

(fn CanOpenSlightlyOpenDoorinTutorial
  (params (TiSiApreInFaccia :type Boolean))
  (if TiSiApreInFaccia
    (for _array_element (Collision|GetOverlappingActors (Variables|Default|GetBox) 0 :!class /Script/Engine.PrimitiveComponent)
      (if (or (Actor|ActorHasTag _array_element "Cart") (Actor|ActorHasTag _array_element "Player"))
        (bind _output_get (LocalVariables|SetCanOpenRoomDoor false))
        (return _output_get)))
    (bind _output_get_2 (LocalVariables|SetCanOpenRoomDoor true))
    (return _output_get_2)
    (else
      (bind _output_get_3 (LocalVariables|SetCanOpenRoomDoor true))
      (return _output_get_3))))