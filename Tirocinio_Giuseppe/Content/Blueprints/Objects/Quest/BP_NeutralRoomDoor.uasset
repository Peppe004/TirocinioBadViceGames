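; Quest-linked hinged room door with separate open/close events for inside and outside, plus a slightly-open tutorial event that unlocks it.
; Timelines lerp the Cardine hinge's yaw, shaking the door instead when it is locked or a trigger zone blocks movement.
; TiSiApreInFaccia adjusts swing angles for the tutorial state and clears after a full swing.
; Interact only forwards quest data and the door to BP_MainGameInstance.QuestAdvanced.
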(event Custom|Door_Slightly_Opens_For_Tutorial
  ;[1 0 0 0.5] Per farla funzionare correttamente durante il tutorial, serve che la porta abbia il tisiapreinfaccia settato a true
  ;;[0.15 0.15 0.15 0.5] La porta si apre leggermente (per il tutorial)
  (bind _output_get (Variables|Rotation|SetTutorialRotationStart (.yaw (Variables|/Script/Engine.SceneComponent|GetRelativeRotation (Variables|Default|GetCardine)))))
  (Variables|Rotation|SetTutorialRotationEnd (+ _output_get 1e+01))
  (Components|Timeline|SetPlayRate (Variables|Default|GetTutorialDoorOpenTimeline) (/ 3.0 1.5))
  (bind _alpha (Timeline|TutorialDoorOpenTimeline PlayFromStart)
    (:Update
      (Transformation|SetRelativeRotation (Variables|Default|GetCardine) (Math|Rotator|MakeRotator 0.0 0.0 (Math|Float|Lerp (Variables|Rotation|GetTutorialRotationStart) (Variables|Rotation|GetTutorialRotationEnd) _alpha)) false false))
    (:Finished
      (Variables|Booleani|SetIsLocked false))))

(event EventOpenCloseDoorfromInsideRoom
  ;[0.15 0.15 0.15 0.5] Apri/chiudi la porta da dentro
  (if (Variables|Booleani|GetIsLocked)
    (if (not (Variables|Booleani|GetIsShaking))
      ;;[1 0 0.6365 0.5] Tremolio se la porta è chiusa a chiave
      (bind _output_get (Variables|Rotation|SetTriggeredRotationStart (.yaw (Variables|/Script/Engine.SceneComponent|GetRelativeRotation (Variables|Default|GetCardine)))))
      (Variables|Rotation|SetTriggeredRotationEnd (Math|Float|Clamp(Float) (+ _output_get 1e+01) -1e+01 1e+01))
      (Variables|Booleani|SetIsShaking true)
      (Components|Timeline|SetPlayRate (Variables|Default|GetTimeline_3) (/ 4.0 0.3))
      (bind _alpha (Timeline|Timeline_3 PlayFromStart)
        (:Update
          (Transformation|SetRelativeRotation (Variables|Default|GetCardine) (Math|Rotator|MakeRotator 0.0 0.0 (Math|Float|Lerp (Variables|Rotation|GetTriggeredRotationStart) (Variables|Rotation|GetTriggeredRotationEnd) _alpha)) false false))
        (:Finished
          (Variables|Booleani|SetIsShaking false))))
    (elif (not (Variables|Booleani|GetIsMoving))
      (if (Variables|Booleani|GetIsOpen)
        (bind _canclose (Default|CanCloseDoor (Variables|Default|GetTriggerZoneForInsideClosing)))
        (if _canclose
          ;;[0 0.5148 1 0.5] Chiudi la porta
          (Variables|Rotation|SetRotationStart (.yaw (Variables|/Script/Engine.SceneComponent|GetRelativeRotation (Variables|Default|GetCardine))))
          (Variables|Rotation|SetRotationEnd (Math|Float|Clamp(Float) (+ (Variables|Rotation|GetRotationStart) (Math|Float|SelectFloat 9e+01 -9e+01 (Variables|Booleani|GetTiSiApreInFaccia))) 0.0 -9e+01))
          (Variables|Booleani|SetIsOpen false)
          (Variables|Booleani|SetIsMoving true)
          ;;[0.7189 0.59 1 0.5] Rotazione porta
          (Components|Timeline|SetPlayRate (Variables|Default|GetTimeline_0) (+ 1.0 0.5) :!label _label)
          (bind _alpha_2 (Timeline|Timeline_0 PlayFromStart)
            (:Update
              (Transformation|SetRelativeRotation (Variables|Default|GetCardine) (Math|Rotator|MakeRotator 0.0 0.0 (Math|Float|Lerp (Variables|Rotation|GetRotationStart) (Variables|Rotation|GetRotationEnd) _alpha_2)) false false))
            (:Finished
              (Variables|Booleani|SetIsMoving false)
              ;;[1 0.5732 0.334 0.5] Abbiamo bisogno che sia true solo se durante il tutorial la porta si è aperta poco e il giocatore la apre per la prima volta
              (if (Variables|Booleani|GetTiSiApreInFaccia)
                (Variables|Booleani|SetTiSiApreInFaccia false))))
          (elif (not (Variables|Booleani|GetIsShaking))
            ;;[0 0 1 0.5] Tremolio per non prendere la porta in faccia quando la chiudiamo
            (bind _output_get_2 (Variables|Rotation|SetTriggeredRotationStart (.yaw (Variables|/Script/Engine.SceneComponent|GetRelativeRotation (Variables|Default|GetCardine)))))
            (Variables|Rotation|SetTriggeredRotationEnd (Math|Float|Clamp(Float) (+ _output_get_2 1e+01) 8e+01 95.0))
            (Variables|Booleani|SetIsShaking true)
            (Components|Timeline|SetPlayRate (Variables|Default|GetTimeline_1) (/ 4.0 0.3))
            (bind _alpha_3 (Timeline|Timeline_1 PlayFromStart)
              (:Update
                (Transformation|SetRelativeRotation (Variables|Default|GetCardine) (Math|Rotator|MakeRotator 0.0 0.0 (Math|Float|Lerp (Variables|Rotation|GetTriggeredRotationStart) (Variables|Rotation|GetTriggeredRotationEnd) _alpha_3)) false false))
              (:Finished
                (Variables|Booleani|SetIsShaking false)))))
        (else
          ;;[0 1 0.198 0.5] Apri la porta
          (bind _output_get_3 (Variables|Rotation|SetRotationStart (.yaw (Variables|/Script/Engine.SceneComponent|GetRelativeRotation (Variables|Default|GetCardine)))))
          (Variables|Rotation|SetRotationEnd (Math|Float|Clamp(Float) (+ _output_get_3 (Math|Float|SelectFloat 8e+01 9e+01 (Variables|Booleani|GetTiSiApreInFaccia))) -9e+01 9e+01))
          (Variables|Booleani|SetIsOpen true)
          (Variables|Booleani|SetIsMoving true)
          (goto _label))))))

(event EventOpenCloseDoorfromOutsideRoom
  ;[0.15 0.15 0.15 0.5] Apri/chiudi porta da fuori
  (if (Variables|Booleani|GetIsLocked)
    (if (not (Variables|Booleani|GetIsShaking)) :!label _label
      ;;[1 0 0.6365 0.5] Tremolio se la porta è chiusa a chiave
      (bind _output_get (Variables|Rotation|SetTriggeredRotationStart (.yaw (Variables|/Script/Engine.SceneComponent|GetRelativeRotation (Variables|Default|GetCardine)))))
      (Variables|Rotation|SetTriggeredRotationEnd (Math|Float|Clamp(Float) (+ _output_get 1e+01) -1e+01 1e+01))
      (Variables|Booleani|SetIsShaking true)
      (Components|Timeline|SetPlayRate (Variables|Default|GetTimeline_4) (/ 4.0 0.3))
      (bind _alpha (Timeline|Timeline_4 PlayFromStart)
        (:Update
          (Transformation|SetRelativeRotation (Variables|Default|GetCardine) (Math|Rotator|MakeRotator 0.0 0.0 (Math|Float|Lerp (Variables|Rotation|GetTriggeredRotationStart) (Variables|Rotation|GetTriggeredRotationEnd) _alpha)) false false))
        (:Finished
          (Variables|Booleani|SetIsShaking false))))
    (elif (not (Variables|Booleani|GetIsMoving))
      (if (Variables|Booleani|GetIsOpen)
        ;;[0.864 0.8049 0 0.5] Controlla se può chiudere la porta
        (bind _canclose (Default|CanCloseDoor (Variables|Default|GetTriggerZoneForOutsideClosing)))
        (if _canclose
          ;;[0 0.5148 1 0.5] Chiudi la porta
          (Variables|Rotation|SetRotationStart (.yaw (Variables|/Script/Engine.SceneComponent|GetRelativeRotation (Variables|Default|GetCardine))))
          (Variables|Rotation|SetRotationEnd (Math|Float|Clamp(Float) (+ (Variables|Rotation|GetRotationStart) (Math|Float|SelectFloat -9e+01 9e+01 (Variables|Booleani|GetTiSiApreInFaccia))) -9e+01 0.0))
          (Variables|Booleani|SetIsOpen false)
          (Variables|Booleani|SetIsMoving true)
          ;;[0.7189 0.59 1 0.5] Rotazione porta
          (Components|Timeline|SetPlayRate (Variables|Default|GetTimeline) (+ 1.0 0.5) :!label _label_2)
          (bind _alpha_2 (Timeline|Timeline PlayFromStart)
            (:Update
              (Transformation|SetRelativeRotation (Variables|Default|GetCardine) (Math|Rotator|MakeRotator 0.0 0.0 (Math|Float|Lerp (Variables|Rotation|GetRotationStart) (Variables|Rotation|GetRotationEnd) _alpha_2)) false false))
            (:Finished
              (Variables|Booleani|SetIsMoving false)
              ;;[1 0.5732 0.334 0.5] Abbiamo bisogno che sia true solo se durante il tutorial la porta si è aperta poco e il giocatore la apre per la prima volta
              (if (Variables|Booleani|GetTiSiApreInFaccia)
                (Variables|Booleani|SetTiSiApreInFaccia false))))
          (elif (not (Variables|Booleani|GetIsShaking))
            ;;[0 0 1 0.5] Tremolio per non prendere la porta in faccia quando la chiudiamo
            (bind _output_get_2 (Variables|Rotation|SetTriggeredRotationStart (.yaw (Variables|/Script/Engine.SceneComponent|GetRelativeRotation (Variables|Default|GetCardine)))))
            (Variables|Rotation|SetTriggeredRotationEnd (Math|Float|Clamp(Float) (+ _output_get_2 1e+01) -8e+01 -9e+01))
            (Variables|Booleani|SetIsShaking true)
            (Components|Timeline|SetPlayRate (Variables|Default|GetTimeline_2) (/ 4.0 0.3))
            (bind _alpha_3 (Timeline|Timeline_2 PlayFromStart)
              (:Update
                (Transformation|SetRelativeRotation (Variables|Default|GetCardine) (Math|Rotator|MakeRotator 0.0 0.0 (Math|Float|Lerp (Variables|Rotation|GetTriggeredRotationStart) (Variables|Rotation|GetTriggeredRotationEnd) _alpha_3)) false false))
              (:Finished
                (Variables|Booleani|SetIsShaking false)))))
        (else
          ;;[0 0 0 0.5] Controlla se può aprire la porta
          (bind _canopen (Default|CanOpenSlightlyOpenDoorinTutorial (Variables|Default|GetTriggerZoneForInsideClosing) (Variables|Booleani|GetTiSiApreInFaccia)))
          (if _canopen
            ;;[0 1 0.198 0.5] Apri la porta
            (bind _output_get_3 (Variables|Rotation|SetRotationStart (.yaw (Variables|/Script/Engine.SceneComponent|GetRelativeRotation (Variables|Default|GetCardine)))))
            (Variables|Rotation|SetRotationEnd (Math|Float|Clamp(Float) (+ _output_get_3 (Math|Float|SelectFloat 9e+01 -9e+01 (Variables|Booleani|GetTiSiApreInFaccia))) -9e+01 9e+01))
            (Variables|Booleani|SetIsOpen true)
            (Variables|Booleani|SetIsMoving true)
            (goto _label_2)
            (else
              (goto _label))))))))

(fn ConstructionScript)

(fn SlightlyOpenShaking
  (bind _output_get (Variables|Rotation|SetTutorialTriggeredRotationStart (.yaw (Variables|/Script/Engine.SceneComponent|GetRelativeRotation (Variables|Default|GetCardine))))))

(fn CheckBinCapacity
  (return false))

(fn DisableCollision
  (return false))

(fn EnableCollision
  (return false))

(fn GetIsOpen
  (return (Variables|Booleani|GetIsOpen)))

(fn GetMesh
  (return 0))

(fn GetQuestID
  (return (Variables|Quest|GetQuest%20ID)))

(fn Interact
  ;[0.15 0.15 0.15 0.5] CALLED BY THE PLAYER WHEN INTERACTING
  (bind _asbp_main_game_instance (Utilities|Casting|CastToBP_MainGameInstance (Game|GetGameInstance)))
  (Default|QuestAdvanced _asbp_main_game_instance (Variables|Quest|GetQuest%20ID) (Variables|Quest|GetCurrent%20Checkpoint) self (Variables|Quest|GetQuestActivationTreshold))
  (return false))

(fn ReturnArrowTransform
  (return ""))

(fn ReturnBinCapacity
  (return 0))

(fn ReturnCleaningType
  (return "NewEnumerator0"))

(fn ReturnTrashInitiaLocation
  (return "0, 0, 0"))

(fn ReturnTrashTravelTransform
  (return ""))

(fn StartDialog
  (return false))

(fn UnlockDoor
  (bind _output_get (Variables|Booleani|SetIsLocked false))
  (return _output_get))