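; BP_QuestObject is an interactable quest object that notifies a door to advance the quest.
; Interact looks up actors sharing its first tag and calls IncrementCheckpointMessage, returning inside the loop after the first match.
; Helper functions turn off the static mesh collision and expose the QuestID.
; The object is call-driven, with BeginPlay, overlap and Tick events disabled.
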(event EventBeginPlay
  (|CallParentFunction) ; Questo nodo è disabilitato e non verrà chiamato.\nTrascina i pin per creare funzionalità.
)

(event Collision|EventActorBeginOverlap
  (params (OtherActor :type Actor%20Object%20Reference))
  (|CallParentFunction OtherActor) ; Questo nodo è disabilitato e non verrà chiamato.\nTrascina i pin per creare funzionalità.
)

(event EventTick
  (params (DeltaSeconds :type Float%20%28single-precision%29))
  (|CallParentFunction DeltaSeconds) ; Questo nodo è disabilitato e non verrà chiamato.\nTrascina i pin per creare funzionalità.
)

(fn ConstructionScript
  (|CallParentFunction))

(fn Interact
  ;[0.15 0.15 0.15 0.5] NOTIFIES DOOR TO ADAVNCE THE QUEST
  (bind _outactors (Actor|GetAllActorswithTag (Utilities|Array|Get(acopy) (Variables|Default|GetTags))))
  (for _array_element _outactors
    (Class|BPIInterarct|IncrementCheckpoint(Message) _array_element)
    (return false)))

(fn DisableCollision
  (Collision|SetCollisionEnabled (Variables|Default|GetStaticMesh) "NoCollision")
  (return false))

(fn GetQuestID
  (return (Variables|Default|GetQuest%20ID)))