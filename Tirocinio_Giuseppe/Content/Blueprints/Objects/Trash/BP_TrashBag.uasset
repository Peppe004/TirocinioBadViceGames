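; BP_TrashBag is a trash bag object that reports its contained trash to the game instance when destroyed.
; On Destroyed it casts to BP_MainGameInstance, passes ContainedTrash to DIsposedObjectUpdate and prints a message about updating the dispose objects quest.
; IncrementContainedTrash is a stub that only returns false, so nothing in this graph changes the contained amount.
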(event EventBeginPlay
  (|CallParentFunction) ; This node is disabled and will not be called.\nDrag off pins to build functionality.
)

(event Collision|EventActorBeginOverlap
  (params (OtherActor :type Actor%20Object%20Reference))
  (|CallParentFunction OtherActor) ; This node is disabled and will not be called.\nDrag off pins to build functionality.
)

(event EventTick
  (params (DeltaSeconds :type Float%20%28single-precision%29))
  (|CallParentFunction DeltaSeconds) ; This node is disabled and will not be called.\nDrag off pins to build functionality.
)

(event EventDestroyed
  (bind _asbp_main_game_instance (Utilities|Casting|CastToBP_MainGameInstance (Game|GetGameInstance)))
  (Default|DIsposedObjectUpdate _asbp_main_game_instance (Variables|Default|GetContained%20Trash%20))
  (Development|PrintString "Updating dispose objects quest "))

(fn ConstructionScript
  (|CallParentFunction))

(fn IncrementContainedTrash
  (return false))