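; Trash bin actor that collects and destroys actors tagged "Trash", counting them against a maximum capacity.
; Collider overlaps send a DestroyTrash message, whose handler increments the count and destroys the item.
; A separate capacity check fires an OnTrashBinIsFull dispatcher at the limit, and a reset event empties the count.
; Helper functions expose the count and collider transform as a trash travel target, and toggle mesh and collider collision.
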(event OnComponentBeginOverlap(Collider)
  (params (OverlappedComponent :type Primitive%20Component%20Object%20Reference) (OtherActor :type Actor%20Object%20Reference) (OtherComp :type Primitive%20Component%20Object%20Reference) (OtherBodyIndex :type Integer) (bFromSweep :type Boolean) (SweepResult :type Hit%20Result%20Structure%20%28by%20ref%29))
  (Class|BPIInterarct|DestroyTrash(Message) self OtherActor))

(event EventBeginPlay)

(event EventResetBinCapacity
  (Variables|Default|SetContained%20Trash 0)
  (Variables|Default|SetIsFull false))

(event EventTick
  (params (DeltaSeconds :type Float%20%28single-precision%29)))

(event EventDestroyTrash
  (params (Trash :type Actor%20Object%20Reference))
  (Utilities|IsValid Trash
    (:Is%20Valid
      (if (Actor|ActorHasTag Trash "Trash")
        (Math|Integer|IncrementInt (Variables|Default|GetContained%20Trash)
          (:%20%20
            (Actor|DestroyActor Trash)))))))

(fn ConstructionScript
  (|CallParentFunction))

(fn ReturnTrashTravelTransform
  (return (Transformation|GetWorldTransform (Variables|Default|GetCollider))))

(fn CheckBinCapacity
  (bind _output_get (LocalVariables|SetTrashBinIsFull (not (<= (Variables|Default|GetContained%20Trash) (- (Variables|Default|GetMax%20Contained%20Trash) 1)))))
  (if _output_get
    (Default|CallOnTrashBinIsFull))
  (return (LocalVariables|GetTrashBinIsFull)))

(fn ReturnBinCapacity
  (return (Variables|Default|GetContained%20Trash)))

(fn DisposeTrash0
  (params (Other%20Actor :type Actor%20Object%20Reference))
  (Utilities|IsValid Other%20Actor
    (:Is%20Valid
      (if (Actor|ActorHasTag Other%20Actor "Trash")
        (Math|Integer|IncrementInt (Variables|Default|GetContained%20Trash)
          (:%20%20
            (Actor|DestroyActor Other%20Actor)))))))

(fn DisableCollision
  (Collision|SetCollisionEnabled (Variables|Default|GetStaticMesh) "NoCollision")
  (Collision|SetCollisionEnabled (Variables|Default|GetCollider) "NoCollision")
  (return false))

(fn EnableCollision
  (Collision|SetCollisionEnabled (Variables|Default|GetStaticMesh) "QueryAndPhysics")
  (Collision|SetCollisionEnabled (Variables|Default|GetCollider) "QueryAndPhysics")
  (return false))

(fn GetMesh
  (return 0))