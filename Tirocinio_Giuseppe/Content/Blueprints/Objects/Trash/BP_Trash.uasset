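; BP_Trash is a trash object that counts toward the game instance's total of objects to dispose of and can be flagged as pickable.
; On BeginPlay it stores its start location, increments that total, then after a short delay notifies the game instance and binds to its TrashCanBePicked event.
; A timeline drives an emissive glow through the lighting component.
; Helper functions toggle collision, halting physics on disable, and expose the mesh, start location and pickable state.
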(event Custom|On_TrashCanBePicked_Event
  ;[0.15 0.15 0.15 0.5] BEGIN PLAY
  (Variables|Default|SetCanBePicked true))

(event EventBeginPlay
  ;[0.15 0.15 0.15 0.5] BEGIN PLAY
  (|CallParentFunction)
  (Variables|Default|SetWorldLocation (Transformation|GetActorLocation))
  (bind _asbp_main_game_instance (Utilities|Casting|CastToBP_MainGameInstance (Game|GetGameInstance)))
  (bind _output_get (Variables|/Game/Blueprints/Singletons/BP_MainGameInstance.BP_MainGameInstance_C|SetTotalObjectsToDispose _asbp_main_game_instance (Variables|/Game/Blueprints/Singletons/BP_MainGameInstance.BP_MainGameInstance_C|GetTotalObjectsToDispose _asbp_main_game_instance)))
  (Math|Integer|IncrementInt _output_get
    (:%20%20
      (Utilities|FlowControl|Delay 0.2)
      (bind _asbp_main_game_instance_2 (Utilities|Casting|CastToBP_MainGameInstance (Game|GetGameInstance)))
      (Default|CommunicatewithTrash _asbp_main_game_instance_2)
      (EventDispatchers|AssignOnTrashCanbePicked _asbp_main_game_instance_2 (delegate Custom|On_TrashCanBePicked_Event)))))

(event EventSetCanbePicked
  (Variables|Default|SetCanBePicked true))

(event EventGlow
  ;[0.15 0.15 0.15 0.5] Si illumina
  (Components|Timeline|SetPlayRate (Variables|Default|GetTrashGlowTimeline) (/ 2.0 2.5))
  (bind _alpha (Timeline|TrashGlowTimeline PlayFromStart)
    (:Update
      (Default|SetValues (Variables|Default|GetBP_LightingComponent) (Math|Float|Lerp (Variables|Default|GetStartEmissive) (Variables|Default|GetEndEmissive) _alpha)))))

(event EventStopGlowing
  ;[0.15 0.15 0.15 0.5] Non si illumina più
  (Audio|Components|Audio|Stop (Variables|Default|GetTrashGlowTimeline))
  (Variables|Default|SetEndEmissive 0.0)
  (Default|SetValues (Variables|Default|GetBP_LightingComponent) 0.0))

(fn ConstructionScript
  (|CallParentFunction))

(fn EnableCollision
  (Collision|SetCollisionEnabled (Variables|Default|GetStaticMesh) "QueryOnly")
  (return false))

(fn DisableCollision
  (Physics|SetSimulatePhysics (Variables|Default|GetStaticMesh) false)
  (Class|PrimitiveComponent|SetAllPhysicsLinearVelocity (Variables|Default|GetStaticMesh) "0, 0, 0" false)
  (Collision|SetCollisionEnabled (Variables|Default|GetStaticMesh) "NoCollision")
  (return false))

(fn ReturnTrashInitiaLocation
  (return (Variables|Default|GetWorldLocation)))

(fn GetMesh
  (return (Variables|Default|GetStaticMesh)))

(fn GetCanbePicked
  (return (Variables|Default|GetCanBePicked)))