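; BP_Incinerator is the trash incinerator that destroys trash bags entering its collider.
; On overlap it stops glowing, destroys any valid actor tagged TrashBag and calls OnTrashBurnt.
; Glow plays a timeline that lerps emissive through the lighting component, while StopGlowing halts it and zeroes the emissive.
; It supplies its mesh transform as the trash travel transform and returns false from Interact and EnableCollision.
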(event OnComponentBeginOverlap(Collider)
  (params (OverlappedComponent :type Primitive%20Component%20Object%20Reference) (OtherActor :type Actor%20Object%20Reference) (OtherComp :type Primitive%20Component%20Object%20Reference) (OtherBodyIndex :type Integer) (bFromSweep :type Boolean) (SweepResult :type Hit%20Result%20Structure%20%28by%20ref%29))
  ;[0.15 0.15 0.15 0.5] TRASH BAG DESTRUCTION
  (CallFunction|DestroyTrash OtherActor))

(event EventBeginPlay
  (|CallParentFunction) ; This node is disabled and will not be called.\nDrag off pins to build functionality.
)

(event EventGlow
  ;[0.15 0.15 0.15 0.5] si illumina
  (Components|Timeline|SetPlayRate (Variables|Default|GetIncineratorTimeline) (/ 2.0 2.5))
  (bind _alpha (Timeline|IncineratorTimeline PlayFromStart)
    (:Update
      (Default|SetValues (Variables|Default|GetBP_LightingComponent) (Math|Float|Lerp (Variables|Default|GetStartEmissive) (Variables|Default|GetEndEmissive) _alpha)))))

(event EventTick
  (params (DeltaSeconds :type Float%20%28single-precision%29))
  (|CallParentFunction DeltaSeconds) ; This node is disabled and will not be called.\nDrag off pins to build functionality.
)

(event EventStopGlowing
  ;[0.15 0.15 0.15 0.5] smette di brillare
  (Audio|Components|Audio|Stop (Variables|Default|GetIncineratorTimeline))
  (Variables|Default|SetEndEmissive 0.0)
  (Default|SetValues (Variables|Default|GetBP_LightingComponent) 0.0))

(event EventDestroyTrash
  (params (Trash :type Actor%20Object%20Reference))
  ;[0.15 0.15 0.15 0.5] TRASH BAG DESTRUCTION
  (Class|BPICleaningTool|StopGlowing(Message) self)
  (bind _output_get (Variables|BasicInteraction|SetOther%20Actor Trash))
  (Utilities|IsValid _output_get
    (:Is%20Valid
      (if (Actor|ActorHasTag _output_get "TrashBag")
        (Actor|DestroyActor (Variables|BasicInteraction|GetOther%20Actor))
        (Default|CallOnTrashBurnt)))))

(fn ConstructionScript
  (|CallParentFunction))

(fn Interact
  (return false))

(fn ReturnTrashTravelTransform
  (return (Transformation|GetWorldTransform (Variables|Default|GetStaticMesh))))

(fn EnableCollision
  (return false))