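; BP_InteractableObject is an interactable world object with placeholder behavior, apparently meant as a base for more specific objects.
; Interact only prints a debug message, while two functions switch the static mesh collision between none and query-only.
; ReturnArrowTransform supplies no computed transform and ReturnCleaningType returns a fixed enum entry.
; The event graph and construction script hold no logic.
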(event EventBeginPlay)

(event Collision|EventActorBeginOverlap
  (params (OtherActor :type Actor%20Object%20Reference)))

(event EventTick
  (params (DeltaSeconds :type Float%20%28single-precision%29)))

(fn ConstructionScript)

(fn DisableCollision
  (Collision|SetCollisionEnabled (Variables|Default|GetStaticMesh) "NoCollision")
  (return false))

(fn EnableCollision
  (Collision|SetCollisionEnabled (Variables|Default|GetStaticMesh) "QueryOnly")
  (return false))

(fn Interact
  (Development|PrintText "Something touched me...")
  (return false))

(fn ReturnArrowTransform
  (return ""))

(fn ReturnCleaningType
  (return "NewEnumerator0"))