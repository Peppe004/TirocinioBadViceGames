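; BP_ElevatorDoor_DX is an elevator door panel that slides open and closed along the world X axis.
; The open event caches the current X, sets the end 60 units further and drives a timeline lerp with teleporting location updates, flagging IsOpening until finished.
; The close event runs a second timeline back to the cached start.
; Play rates stretch both timelines by 2.5.
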(event Custom|Open_Elevator_Door_DX
  (bind _returnvalue (Transformation|GetActorLocation))
  ;[0.15 0.15 0.15 0.5] apre
  (bind _output_get (Variables|Default|SetStartLocation (.x (Transformation|GetActorLocation))))
  (Variables|Default|SetEndLocation (+ _output_get 6e+01))
  (Variables|Default|SetIsOpening true)
  (Components|Timeline|SetPlayRate (Variables|Default|GetOpening_Timeline) (/ 1.0 2.5))
  (bind _alpha (Timeline|Opening_Timeline PlayFromStart)
    (:Update
      (Transformation|SetActorLocation (Math|Vector|MakeVector (Math|Float|Lerp (Variables|Default|GetStartLocation) (Variables|Default|GetEndLocation) _alpha) (.y _returnvalue) (.z _returnvalue)) false true))
    (:Finished
      (Variables|Default|SetIsOpening false))))

(event Custom|Close_Elevator_Door_DX
  (bind _returnvalue (Transformation|GetActorLocation))
  ;[0.15 0.15 0.15 0.5] chiude
  (Components|Timeline|SetPlayRate (Variables|Default|GetClosing_Timeline) (/ 1.0 2.5))
  (bind _alpha (Timeline|Closing_Timeline PlayFromStart)
    (:Update
      (Transformation|SetActorLocation (Math|Vector|MakeVector (Math|Float|Lerp (Variables|Default|GetEndLocation) (Variables|Default|GetStartLocation) _alpha) (.y _returnvalue) (.z _returnvalue)) false true))))

(fn ConstructionScript)