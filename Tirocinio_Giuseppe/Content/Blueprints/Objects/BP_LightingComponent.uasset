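; BP_LightingComponent is a component that controls the emissive strength of its owning actor's static meshes.
; On BeginPlay it creates dynamic material instances for every material slot on each of the owner's static mesh components and stores them.
; Set_values pushes a given value into the Emissive scalar parameter of all stored instances.
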(event Custom|Set_values
  (params (EmissiveParameter :type Float%20%28double-precision%29))
  (for _array_element (Variables|Default|GetMaterialInstance)
    (Rendering|Material|SetScalarParameterValue _array_element "Emissive" EmissiveParameter :!class /Script/Engine.MaterialInstanceDynamic)))

(event EventBeginPlay
  (for _array_element (Actor|GetComponentsByClass (Components|GetOwner) "/Script/Engine.StaticMeshComponent")
    (for (_array_element_2 _array_index) (Rendering|Material|GetMaterials _array_element)
      (bind _returnvalue (Rendering|Material|CreateDynamicMaterialInstance _array_element _array_index _array_element_2 "None" :!class /Script/Engine.PrimitiveComponent))
      (Utilities|Array|Add (Variables|Default|GetMaterialInstance) _returnvalue))))

(event EventTick
  (params (DeltaSeconds :type Float%20%28single-precision%29)))