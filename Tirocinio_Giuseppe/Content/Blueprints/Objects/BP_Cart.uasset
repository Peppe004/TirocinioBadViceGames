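; Possessable cleaning cart pawn the player pushes around, with a bin child actor and attach points for tools sorted by tag.
; Player controller events drive scaled movement, yaw-based turning and sphere-trace door interaction, with idle/walk camera shakes.
; Detaching repossesses the original pawn at a spot found by downward traces behind, right, then left, rejecting Wall-tagged hits.
; A timeline can turn the cart toward a focus object, then unlock input and allow detaching.
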(event Custom|Move_Forward
  (params (Move_Forward_Value :type Float%20%28double-precision%29))
  ;[0.15 0.15 0.15 0.5] Move forward and right
  (bind _newparam (CallFunction|GetCanMove))
  (if _newparam
    (Pawn|Input|AddMovementInput (Transformation|GetActorForwardVector) (/ Move_Forward_Value 4.0) false)))

(event Custom|Look
  (params (NewParam :type Vector%202D%20Structure))
  (bind (_x _y) (Math|Vector2D|BreakVector2D NewParam))
  ;[0.15 0.15 0.15 0.5] Mouse movement
  (if (== (Game|Player|GetPlayerPawn 0) self)
    (Variables|Default|SetCart_Rotation (+ (Variables|Default|GetCart_Rotation) (* _x 1.0)))
    (Pawn|Input|AddControllerPitchInput (* _y -1.0))))

(event Custom|Move_Right_Value
  (params (Move_Right_Value :type Float%20%28double-precision%29))
  ;[0.15 0.15 0.15 0.5] Move forward and right
  (bind _newparam (CallFunction|GetCanMove))
  (if _newparam
    (Pawn|Input|AddMovementInput (Transformation|GetActorRightVector) (/ Move_Right_Value 2.7) false)))

(event Custom|OnDetach
  ;[0.15 0.15 0.15 0.5] Staccati dal cart e riprendi controllo del player
  (if (Variables|Default|GetCanDetach)
    (Utilities|IsValid (Variables|Default|GetOldPawn)
      (:Is%20Valid
        (bind _playerposition (CallFunction|TracetoSpawnPlayer))
        (Transformation|SetActorLocation (Variables|Default|GetOldPawn) _playerposition false false)
        (Class|BPIInterarct|EnableCollision(Message) (Variables|/Script/Engine.ChildActorComponent|GetChildActor (Variables|Default|GetBin)))
        (Pawn|Possess (Variables|Default|GetPlayerController) (Variables|Default|GetOldPawn))
        (Class|BPIPlayer|ResetUICollider(Message) (Variables|Default|GetOldPawn))
        (Collision|SetCollisionResponsetoChannel (Variables|Default|GetOldPawnCollider) "ECC_Pawn" "ECR_Block")
        (Pawn|SetControlRotation (Variables|Default|GetPlayerController) (Transformation|GetWorldRotation (Variables|Default|GetPlayerPositionWhileHoldingCart)))
        (Variables|Default|SetOldPawn 0)
        (Variables|Default|SetOldPawnCollider 0)))))

(event Custom|Interact_Event
  ;[0.15 0.15 0.15 0.5] Interact
  (if (== (Game|Player|GetPlayerPawn 0) self)
    (CallFunction|Trace)))

(event Custom|Camera_Shakes
  (bind _returnvalue (Game|GetPlayerController 0))
  ;[0.15 0.15 0.15 0.5] Camera Shakes Idle Walk
  (if (> (Math|Vector|VectorLength (Transformation|GetVelocity)) 0.0)
    (Game|Feedback|ClientStartCameraShake _returnvalue "/Game/Blueprints/Objects/CameraShakes/BP_WalkCameraShakes.BP_WalkCameraShakes_C" 1.0 "CameraLocal" "0, 0, 0")
    (else
      (Game|Feedback|ClientStartCameraShake _returnvalue "/Game/Blueprints/Objects/CameraShakes/BP_IdleCameraShakes.BP_IdleCameraShakes_C" 1.0 "CameraLocal" "0, 0, 0"))))

(event EventBeginPlay
  ;[0.15 0.15 0.15 0.5] Binding
  (bind _asplayer_controller_bp (Utilities|Casting|CastToPlayerControllerBP (Game|GetPlayerController 0)))
  (Variables|Default|SetPlayerController _asplayer_controller_bp)
  (EventDispatchers|BindEventtoMoveForward (Variables|Default|GetPlayerController) (EventDispatchers|CreateEvent :!event Custom|Move_Forward))
  (EventDispatchers|BindEventtoMoveRight (Variables|Default|GetPlayerController) (EventDispatchers|CreateEvent :!event Custom|Move_Right_Value))
  (EventDispatchers|BindEventtoLook (Variables|Default|GetPlayerController) (EventDispatchers|CreateEvent :!event Custom|Look))
  (EventDispatchers|BindEventtoDetach (Variables|Default|GetPlayerController) (EventDispatchers|CreateEvent :!event Custom|OnDetach))
  (EventDispatchers|BindEventtoInteract (Variables|Default|GetPlayerController) (EventDispatchers|CreateEvent :!event Custom|Interact_Event))
  (Variables|Default|SetCart_Rotation (.yaw (Transformation|GetActorRotation))))

(event EventGetOriginalPlayer
  (params (OriginalPlayer :type Pawn%20Object%20Reference))
  ;[0.15 0.15 0.15 0.5] Prendo il riferimento al player prima del possess
  (bind _output_get (Variables|Default|SetOldPawn OriginalPlayer))
  (bind _playercollider (Class|BPIPlayer|GetCapsuleComponent(Message) _output_get))
  (Variables|Default|SetOldPawnCollider _playercollider))

(event EventTick
  (params (DeltaSeconds :type Float%20%28single-precision%29))
  (Transformation|SetActorRotation (Math|Rotator|MakeRotator 0.0 0.0 (Variables|Default|GetCart_Rotation)))
  (CallFunction|CameraShakes))

(event EventDisableBinCollision
  (Class|BPIInterarct|DisableCollision(Message) (Variables|/Script/Engine.ChildActorComponent|GetChildActor (Variables|Default|GetBin))))

(event EventLockMovement
  ;[0.15 0.15 0.15 0.5] Lock/unlock basic inputs
  (Variables|/Game/Blueprints/PlayerControllerBP.PlayerControllerBP_C|SetCanMove (Variables|Default|GetPlayerController) false))

(event EventUnlockMovement
  ;[0.15 0.15 0.15 0.5] Lock/unlock basic inputs
  (Variables|/Game/Blueprints/PlayerControllerBP.PlayerControllerBP_C|SetCanMove (Variables|Default|GetPlayerController) true))

(event EventUnlockVision
  ;[0.15 0.15 0.15 0.5] Lock/unlock basic inputs
  (Variables|/Game/Blueprints/PlayerControllerBP.PlayerControllerBP_C|SetCanLook (Variables|Default|GetPlayerController) true))

(event EventLockVision
  ;[0.15 0.15 0.15 0.5] Lock/unlock basic inputs
  (Variables|/Game/Blueprints/PlayerControllerBP.PlayerControllerBP_C|SetCanLook (Variables|Default|GetPlayerController) false))

(event EventRotatetoObject
  (params (FocusObject :type Actor%20Object%20Reference))
  (bind _returnvalue (Transformation|GetActorLocation FocusObject))
  (bind _returnvalue_2 (Game|GetPlayerCameraManager 0))
  (bind _returnvalue_3 (Transformation|GetActorLocation FocusObject))
  (bind _returnvalue_4 (Game|GetPlayerCameraManager 0))
  (bind _returnvalue_5 (Pawn|GetControlRotation :!class /Script/Engine.Pawn))
  (bind _returnvalue_6 (Camera|GetCameraLocation _returnvalue_2))
  (bind _returnvalue_7 (Camera|GetCameraLocation _returnvalue_4))
  ;[0.15 0.15 0.15 0.5] Ti giri verso un pnto specifico
  (Variables|Default|SetCurrentRoll (.roll _returnvalue_5))
  (Variables|Default|SetCurrentPitch (.pitch _returnvalue_5))
  (Variables|Default|SetStartRotation (Camera|GetCameraRotation _returnvalue_4))
  (Variables|Default|SetTargetRotation (Math|Rotator|FindLookatRotation (Math|Vector|MakeVector (.x _returnvalue_7) (.y _returnvalue_7) (.z _returnvalue_7)) (Math|Vector|MakeVector (.x _returnvalue_3) (.y _returnvalue_3) (.z _returnvalue_7))))
  (Components|Timeline|SetPlayRate (Variables|Default|GetRotationToPoint_Timeline) (/ 1.0 2.5))
  (bind _alpha (Timeline|RotationToPoint_Timeline PlayFromStart)
    (:Update
      (Variables|Default|SetCart_Rotation (.yaw (Math|Rotator|Lerp(Rotator) (Math|Rotator|MakeRotator 0.0 0.0 (.yaw (Variables|Default|GetStartRotation))) (Math|Rotator|MakeRotator 0.0 0.0 (.yaw (Math|Rotator|FindLookatRotation (Math|Vector|MakeVector (.x _returnvalue_6) (.y _returnvalue_6) (.z _returnvalue_6)) (Math|Vector|MakeVector (.x _returnvalue) (.y _returnvalue) (.z _returnvalue_6))))) _alpha true))))
    (:Finished
      (Utilities|FlowControl|Delay 2.0)
      (CallFunction|UnlockMovement)
      (CallFunction|UnlockVision)
      (Variables|Default|SetCanDetach true))))

(fn ConstructionScript)

(fn Trace
  (bind _cinecamera (Variables|Default|GetCineCamera))
  (bind _returnvalue (Transformation|GetWorldLocation _cinecamera))
  (bind _outhit (Collision|SphereTraceByChannel _returnvalue (+ _returnvalue (* (Math|Vector|GetForwardVector _cinecamera) (LocalVariables|GetRayCastDistance))) 8.0 "TraceTypeQuery1" false (Variables|Default|GetObjectsToIgnoreWithTrace) "ForDuration"))
  (LocalVariables|SetHit_Actor (.HitActor (Collision|BreakHitResult _outhit)))
  (bind _output_get (LocalVariables|SetHit_Component (.HitComponent (Collision|BreakHitResult _outhit))))
  (Utilities|IsValid _output_get
    (:Is%20Valid
      ;[0.15 0.15 0.15 0.5] Porte
      (if (Components|ComponentHasTag (LocalVariables|GetHit_Component) (Variables|Default|GetRoomDoorFromOutsideTag))
        (Class|BPIInterarct|OpenCloseDoorfromOutsideRoom(Message) (LocalVariables|GetHit_Actor))
        (elif (Components|ComponentHasTag (LocalVariables|GetHit_Component) (Variables|Default|GetRoomDoorFromInsideTag))
          (Class|BPIInterarct|OpenCloseDoorfromInsideRoom(Message) (LocalVariables|GetHit_Actor)))))))

(fn TracetoSpawnPlayer
  (bind _playerpositionwhileholdingcart (Variables|Default|GetPlayerPositionWhileHoldingCart))
  (bind _playerpositionwhileholdingcartdx (Variables|Default|GetPlayerPositionWhileHoldingCartDX))
  (bind _playerpositionwhileholdingcartsx (Variables|Default|GetPlayerPositionWhileHoldingCartSX))
  (bind _returnvalue (Transformation|GetWorldLocation _playerpositionwhileholdingcartsx))
  (bind _returnvalue_2 (Transformation|GetWorldLocation _playerpositionwhileholdingcartdx))
  (bind _returnvalue_3 (Transformation|GetWorldLocation _playerpositionwhileholdingcart))
  (bind (_outhit _returnvalue_4) (Collision|SphereTraceByChannel _returnvalue_3 (+ _returnvalue_3 (* (Math|Vector|GetUpVector _playerpositionwhileholdingcart) "0.000000,0.000000,-1.000000" (LocalVariables|GetRayCastDistance))) 45.0 "TraceTypeQuery3" false 0 "None"))
  (if _returnvalue_4
    (if (Actor|ActorHasTag (.HitActor (Collision|BreakHitResult _outhit)) "Wall")
      _
      (else
        (return (.Location (Collision|BreakHitResult _outhit))))))
  (bind (_outhit_2 _returnvalue_5) (Collision|SphereTraceByChannel _returnvalue_2 (+ _returnvalue_2 (* (Math|Vector|GetUpVector _playerpositionwhileholdingcartdx) "0.000000,0.000000,-1.000000" (LocalVariables|GetRayCastDistance))) 45.0 "TraceTypeQuery3" false 0 "None"))
  (if _returnvalue_5
    (if (Actor|ActorHasTag (.HitActor (Collision|BreakHitResult _outhit_2)) "Wall")
      _
      (else
        (return (.Location (Collision|BreakHitResult _outhit_2))))))
  (bind (_outhit_3 _returnvalue_6) (Collision|SphereTraceByChannel _returnvalue (+ _returnvalue (* (Math|Vector|GetUpVector _playerpositionwhileholdingcartsx) "0.000000,0.000000,-1.000000" (LocalVariables|GetRayCastDistance))) 45.0 "TraceTypeQuery3" false 0 "None"))
  (if _returnvalue_6
    (if (not (Actor|ActorHasTag (.HitActor (Collision|BreakHitResult _outhit_3)) "Wall"))
      (return (.Location (Collision|BreakHitResult _outhit_3))))))

(fn CheckBinCapacity
  (return false))

(fn DisableCollision
  (return false))

(fn EnableCollision
  (return false))

(fn GetCanMove
  (return (Variables|Default|GetcanMove)))

(fn GetCanTakeTrashBag
  (return false))

(fn GetCapsuleComponent
  (return 0))

(fn GetIsOpen
  (return false))

(fn GetMesh
  (return 0))

(fn GetObjectstoIgnorewithTrace
  (return (Variables|Default|GetObjectsToIgnoreWithTrace)))

(fn GetQuestID
  (return "None"))

(fn Interact)

(fn PutObjectonCart
  (params (HeldObject :type Actor%20Object%20Reference))
  (bind _output_get (LocalVariables|SetObjectInHand HeldObject))
  (Utilities|IsValid _output_get
    (:Is%20Valid
      (for _array_element (Variables|/Script/Engine.Actor|GetTags HeldObject)
        (switch name _array_element
          (:Mop
            (Transformation|AttachComponentToComponent HeldObject (Variables|Default|GetMopAttachmentPoint) "None" "SnapToTarget" "SnapToTarget" "SnapToTarget" true))
          (:Duster
            (Transformation|AttachComponentToComponent HeldObject 0 "None" "SnapToTarget" "SnapToTarget" "SnapToTarget" true))
          (:Swatter
            (Transformation|AttachComponentToComponent HeldObject (Variables|Default|GetSwatterAttachmentPoint) "None" "SnapToTarget" "SnapToTarget" "KeepRelative" true)))
        (LocalVariables|SetObjectInHand 0)
        (return false)))))

(fn ReturnArrowTransform
  (return ""))

(fn ReturnBinCapacity
  (return 0))

(fn ReturnCleaningType
  (return "NewEnumerator0"))

(fn ReturnCurrentHeldObject
  (return 0))

(fn ReturnTrashInitiaLocation
  (return "0, 0, 0"))

(fn ReturnTrashTravelTransform
  (return ""))

(fn SetCanMove
  (params (Can_Move :type Boolean))
  (Variables|Default|SetcanMove Can_Move)
  (return))

(fn SetCartCollision
  (params (Collision :type ECollisionEnabled%20Enum :default "NoCollision"))
  (return false))

(fn SetCartCollisionResponsetoChannel
  (params (Channel :type ECollisionChannel%20Enum :default "ECC_WorldStatic") (CollisionResponse :type ECollisionResponse%20Enum :default "ECR_Ignore"))
  (return "NoCollision"))

(fn SetObjectstoIgnorewithTrace
  (params (Object :type Actor%20Object%20Reference))
  (Utilities|Array|Add (Variables|Default|GetObjectsToIgnoreWithTrace) Object)
  (return 0))

(fn StartDialog
  (return false))

(fn UnlockDoor
  (return false))