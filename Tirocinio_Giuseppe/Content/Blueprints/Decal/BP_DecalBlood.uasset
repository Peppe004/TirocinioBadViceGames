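; BP_DecalBlood is a blood stain decal actor whose opacity can be stepped down to clean it or up to intensify it.
; BeginPlay creates a dynamic material instance on the decal and sets the tracked opacity to its maximum.
; CleanStain lowers the Opacity parameter by a fixed step and destroys the actor at zero or below.
; MakeStainBigger raises opacity by the same step while below maximum, leaving decal size unchanged.
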(event EventBeginPlay
  (bind _returnvalue (Rendering|Material|CreateDynamicMaterialInstance (Variables|Default|GetDecal) :!class /Script/Engine.DecalComponent))
  (Variables|Default|SetMaterial _returnvalue)
  (Variables|Default|SetCurrentOpacity (Variables|Default|GetMaxOpacity)))

(event Collision|EventActorBeginOverlap
  (params (OtherActor :type Actor%20Object%20Reference)))

(event EventMakeStainBigger
  (bind _returnvalue (Rendering|Material|GetScalarParameterValue (Variables|Default|GetMaterial) "Opacity" :!class /Script/Engine.MaterialInstanceDynamic))
  (if (< _returnvalue (Variables|Default|GetMaxOpacity))
    (bind _output_get (Variables|Default|SetCurrentOpacity (+ (Variables|Default|GetCurrentOpacity) (Variables|Default|GetOpacityToBeSubtract))))
    (Rendering|Material|SetScalarParameterValue (Variables|Default|GetMaterial) "Opacity" _output_get :!class /Script/Engine.MaterialInstanceDynamic)))

(event EventCleanStain
  (Rendering|Material|SetScalarParameterValue (Variables|Default|GetMaterial) "Opacity" (- (Variables|Default|GetCurrentOpacity) (Variables|Default|GetOpacityToBeSubtract)) :!class /Script/Engine.MaterialInstanceDynamic)
  (bind _returnvalue (Rendering|Material|GetScalarParameterValue (Variables|Default|GetMaterial) "Opacity" :!class /Script/Engine.MaterialInstanceDynamic))
  (bind _output_get (Variables|Default|SetCurrentOpacity _returnvalue))
  (if (<= _output_get 0.0)
    (Actor|DestroyActor)))

(fn ConstructionScript)