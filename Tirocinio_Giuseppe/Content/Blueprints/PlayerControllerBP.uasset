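; Player controller Blueprint that turns Enhanced Input into move, look, interact, use-tool and detach calls.
; On BeginPlay it adds the player input mapping context, then relays each action through what appear to be event dispatchers, leaving gameplay response to listeners.
; CanMove and CanLook gate movement and camera input, and look Y is inverted before forwarding.
; Interact, tool use and detach pass through ungated.
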(event Input|EnhancedActionEvents|EnhancedInputActionIA_Detach
  (params (ActionValue :type Boolean) (ElapsedSeconds :type Float%20%28double-precision%29) (TriggeredSeconds :type Float%20%28double-precision%29) (InputAction :type Input%20Action%20Object%20Reference :default "/Game/Input/Actions/IA_Detach.IA_Detach"))
  (Default|CallDetach))

(event Input|EnhancedActionEvents|EnhancedInputActionIA_Look
  (params (ActionValue :type Vector%202D%20Structure) (ElapsedSeconds :type Float%20%28double-precision%29) (TriggeredSeconds :type Float%20%28double-precision%29) (InputAction :type Input%20Action%20Object%20Reference :default "/Game/Input/Actions/IA_Look.IA_Look"))
  (bind (_x _y) (Math|Vector2D|BreakVector2D ActionValue))
  (if (Variables|Default|GetCanLook)
    (Default|CallLook (Math|Vector2D|MakeVector2D _x (* _y -1.0)))))

(event Input|EnhancedActionEvents|EnhancedInputActionIA_Interact
  (params (ActionValue :type Boolean) (ElapsedSeconds :type Float%20%28double-precision%29) (TriggeredSeconds :type Float%20%28double-precision%29) (InputAction :type Input%20Action%20Object%20Reference :default "/Game/Input/Actions/IA_Interact.IA_Interact"))
  (:Started
    (Default|CallInteract)))

(event Input|EnhancedActionEvents|EnhancedInputActionIA_Use_Tool
  (params (ActionValue :type Boolean) (ElapsedSeconds :type Float%20%28double-precision%29) (TriggeredSeconds :type Float%20%28double-precision%29) (InputAction :type Input%20Action%20Object%20Reference :default "/Game/Input/Actions/IA_Use_Tool.IA_Use_Tool"))
  (:Started
    (Default|CallUseTool)))

(event Input|EnhancedActionEvents|EnhancedInputActionIA_Move_Forward
  (params (ActionValue :type Float%20%28double-precision%29) (ElapsedSeconds :type Float%20%28double-precision%29) (TriggeredSeconds :type Float%20%28double-precision%29) (InputAction :type Input%20Action%20Object%20Reference :default "/Game/Input/Actions/IA_Move_Forward.IA_Move_Forward"))
  (if (Variables|Default|GetCanMove)
    (Default|CallMoveForward ActionValue)))

(event Input|EnhancedActionEvents|EnhancedInputActionIA_Move_Right
  (params (ActionValue :type Float%20%28double-precision%29) (ElapsedSeconds :type Float%20%28double-precision%29) (TriggeredSeconds :type Float%20%28double-precision%29) (InputAction :type Input%20Action%20Object%20Reference :default "/Game/Input/Actions/IA_Move_Right.IA_Move_Right"))
  (if (Variables|Default|GetCanMove)
    (Default|CallMoveRight ActionValue)))

(event EventBeginPlay
  (bind _returnvalue (PlayerController|LocalPlayerSubsystems|GetEnhancedInputLocalPlayerSubsystem))
  (Utilities|IsValid _returnvalue
    (:Is%20Valid
      (Input|AddMappingContext _returnvalue "/Game/Input/IMC_PlayerInput.IMC_PlayerInput" 0 "(bIgnoreAllPressedKeysUntilRelease=True,bForceImmediately=False,bNotifyUserSettings=False)"))))

(fn ConstructionScript)