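; Killable cockroach that wanders at random and scurries faster while the player is inside its trigger area.
; A looping timeline lerps it toward random reachable points nearby, turned to face each one, with play rate chosen per move.
; It registers with the main game instance on spawn, exposes cleaning-tool matching and hit points, and is destroyed at zero.
; On destruction it reports the kill and sphere-traces downward to spawn a surface-aligned blood stain.
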(event OnComponentBeginOverlap(TriggerArea)
  (params (OverlappedComponent :type Primitive%20Component%20Object%20Reference) (OtherActor :type Actor%20Object%20Reference) (OtherComp :type Primitive%20Component%20Object%20Reference) (OtherBodyIndex :type Integer) (bFromSweep :type Boolean) (SweepResult :type Hit%20Result%20Structure%20%28by%20ref%29))
  ;[0.15 0.15 0.15 0.5] Controllo se il player entra o esce dalla zona di trigger
  (if (== OtherActor (Game|Player|GetPlayerPawn 0))
    (Variables|Default|SetPlayerIsInTriggerArea true)))

(event OnComponentEndOverlap(TriggerArea)
  (params (OverlappedComponent :type Primitive%20Component%20Object%20Reference) (OtherActor :type Actor%20Object%20Reference) (OtherComp :type Primitive%20Component%20Object%20Reference) (OtherBodyIndex :type Integer))
  ;[0.15 0.15 0.15 0.5] Controllo se il player entra o esce dalla zona di trigger
  (if (== OtherActor (Game|Player|GetPlayerPawn 0))
    (Variables|Default|SetPlayerIsInTriggerArea false)))

(event Custom|Choose_A_New_Location
  ;[0.15 0.15 0.15 0.5] Lo scarafaggio si muove a caso e si gira verso dove si sta muovendo
  (Variables|Default|SetCurrentTrasform (Transformation|GetActorTransform))
  (Variables|Default|SetRandom%20Location (.RandomLocation (AI|Navigation|GetRandomReachablePointinRadius (Transformation|GetActorLocation) 2.5e+02 0 0)))
  (Variables|Default|SetTargetTransform (Math|Transform|MakeTransform (Math|Vector|MakeVector (.X (Math|Vector|BreakVector (Variables|Default|GetRandom%20Location))) (.Y (Math|Vector|BreakVector (Variables|Default|GetRandom%20Location))) (.Z (Math|Vector|BreakVector (Transformation|GetActorLocation)))) (Math|Rotator|MakeRotator 0.0 0.0 (.yaw (Math|Rotator|FindLookatRotation (Transformation|GetActorLocation) (Variables|Default|GetRandom%20Location)))) "1.000000,1.000000,1.000000"))
  (Components|Timeline|SetPlayRate (Variables|Default|GetCockroachTimeLine) (/ 1.0 (Math|Float|SelectFloat 0.25 1.0 (Variables|Default|GetPlayerIsInTriggerArea))))
  (bind _alpha (Timeline|CockroachTimeLine PlayFromStart)
    (:Update
      (Transformation|SetActorTransform (Math|Transform|Lerp(Transform) (Variables|Default|GetCurrentTrasform) (Variables|Default|GetTargetTransform) _alpha) false true))
    (:Finished
      (CallFunction|ChooseANewLocation))))

(event EventBeginPlay
  (CallFunction|ChooseANewLocation)
  (bind _asbp_main_game_instance (Utilities|Casting|CastToBP_MainGameInstance (Game|GetGameInstance)))
  (Math|Integer|IncrementInt (Variables|/Game/Blueprints/Singletons/BP_MainGameInstance.BP_MainGameInstance_C|GetTotalCockroachesToKill _asbp_main_game_instance)))

(event EventDestroyed
  (bind _asbp_main_game_instance (Utilities|Casting|CastToBP_MainGameInstance (Game|GetGameInstance)))
  (Default|KilledCockroachedUpdate _asbp_main_game_instance)
  (CallFunction|SpawnStainatDeath))

(fn ConstructionScript)

(fn SpawnStainatDeath
  (bind _self self)
  (bind _returnvalue (Transformation|GetActorLocation _self))
  (bind _outhit (Collision|SphereTraceByChannel _returnvalue (+ _returnvalue (* (Transformation|GetActorUpVector _self) -200)) 5.0 "TraceTypeQuery1" false 0 "ForDuration" true "(R=1.000000,G=0.000000,B=0.000000,A=1.000000)" "(R=0.000000,G=1.000000,B=0.000000,A=1.000000)" 2e+01))
  (Game|SpawnActorfromClass "/Game/Blueprints/Objects/CleanableObjects/BP_BloodStain.BP_BloodStain_C" (Math|Transform|MakeTransform (.Location (Collision|BreakHitResult _outhit)) (Math|Conversions|RotationFromXVector (.Normal (Collision|BreakHitResult _outhit))) "1.000000,1.000000,1.000000") "Undefined" "MultiplyWithRoot" 0 0)
  (bind _asbp_main_game_instance (Utilities|Casting|CastToBP_MainGameInstance (Game|GetGameInstance)))
  (Default|OnSpawnStain _asbp_main_game_instance))

(fn CheckBinCapacity
  (return false))

(fn DisableCollision
  (return false))

(fn EnableCollision
  (return false))

(fn GetIsOpen
  (return false))

(fn GetMesh
  (return 0))

(fn GetQuestID
  (return "None"))

(fn Interact
  (return false))

(fn MatchesEnum
  (params (Tool :type Actor%20Object%20Reference))
  (bind _newparam (Class|BPIInterarct|ReturnCleaningType(Message) Tool))
  (return (== (Math|Byte|MakeLiteralByte _newparam) (Math|Byte|MakeLiteralByte (Variables|Default|GetType)))))

(fn ReturnArrowTransform
  (return ""))

(fn ReturnBinCapacity
  (return 0))

(fn ReturnCleaningType
  (return (Variables|Default|GetType)))

(fn ReturnTrashInitiaLocation
  (return "0, 0, 0"))

(fn ReturnTrashTravelTransform
  (return ""))

(fn StartDialog
  (return false))

(fn SubtractHitPoints
  (bind _output_get (Variables|Default|SetHit%20Points (- (Variables|Default|GetHit%20Points) 1)))
  (if (== _output_get 0)
    (Actor|DestroyActor)
    (else
      (return false))))

(fn UnlockDoor
  (return false))