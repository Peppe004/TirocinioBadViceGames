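; BP_NotInteractableCockroach is a decorative cockroach actor that scurries from its spot to a given target point, apparently to leave the room, then destroys itself.
; The Cockroach_Go_Out_of_The_Room event stores the start location and plays a timeline.
; Each update lerps toward the target, adds a zigzag offset along the path's right vector, and turns the actor to face that position before moving it without sweep.
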(event Custom|Cockroach_Go_Out_of_The_Room
  (params (TargetPoint :type Actor%20Object%20Reference))
  (Variables|Default|SetTarget%20Point TargetPoint)
  (Variables|Default|SetCurrentLocation (Transformation|GetActorLocation))
  (bind (_direction _alpha _zigzagalpha) (Timeline|NotInteractableCockroachTimeLine PlayFromStart)
    (:Update
      (Transformation|SetActorRotation (Math|Rotator|FindLookatRotation (Transformation|GetActorLocation) (+ (Math|Vector|Lerp(Vector) (Variables|Default|GetCurrentLocation) (Transformation|GetActorLocation (Variables|Default|GetTarget%20Point)) _alpha) (* _zigzagalpha (Math|Vector|GetRightVector (Math|Rotator|FindLookatRotation (Variables|Default|GetCurrentLocation) (Transformation|GetActorLocation (Variables|Default|GetTarget%20Point))))))))
      (Transformation|SetActorLocation (+ (Math|Vector|Lerp(Vector) (Variables|Default|GetCurrentLocation) (Transformation|GetActorLocation (Variables|Default|GetTarget%20Point)) _alpha) (* _zigzagalpha (Math|Vector|GetRightVector (Math|Rotator|FindLookatRotation (Variables|Default|GetCurrentLocation) (Transformation|GetActorLocation (Variables|Default|GetTarget%20Point)))))) false false))
    (:Finished
      (Actor|DestroyActor))))

(fn ConstructionScript)