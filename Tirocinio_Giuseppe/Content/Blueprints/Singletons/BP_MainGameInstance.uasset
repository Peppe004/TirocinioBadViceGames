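; Game instance that holds cleaning, disposal and customer quest progress and owns the HUD widgets.
; Update events advance the cleaned and disposed counters, refresh the objective list, and flag main quests finished when called at or past their totals.
; QuestAdvanced forwards checkpoints to the quest manager, then reads the quest map by index to flag Serial Killer, Drug Dealer or Gang Member completion.
; It also creates and relays updates to objective list and input prompt widgets.
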(event Custom|QuestAdvanced
  (params (Quest%20ID :type Name) (Checkpoints :type Integer) (Door :type Actor%20Object%20Reference) (QuestActivationTreshold :type Integer))
  ;[0.15 0.15 0.15 0.5] UPDATING CHARACTERS QUESTS STATES, CALLED BY IN-GAME OBJECTS
  (Utilities|IsValid (Variables|Default|GetQuest%20Manager%20Ref)
    (:Is%20Valid
      (Default|UpdateQuest (Variables|Default|GetQuest%20Manager%20Ref) Door Checkpoints QuestActivationTreshold)
      (Utilities|Map|Add (Variables|Progression|GetCustomerQuestsMap) Quest%20ID Checkpoints)
      (if (== (.Value (Utilities|Map|GetKeyValueByIndex (Variables|Progression|GetCustomerQuestsMap) 0)) 2)
        (Utilities|Map|Add (Variables|Progression|GetMainQuestsMap) "FinishedQuestSerialKiller" true)
        (Development|PrintText "Serial Killer door opening...")
        (elif (== (.Value (Utilities|Map|GetKeyValueByIndex (Variables|Progression|GetCustomerQuestsMap) 1)) 2)
          (Utilities|Map|Add (Variables|Progression|GetMainQuestsMap) "FinishedQuestDrugDealer" true)
          (Development|PrintText "Drug Dealer door opening...")
          (elif (== (.Value (Utilities|Map|GetKeyValueByIndex (Variables|Progression|GetCustomerQuestsMap) 2)) 2)
            (Utilities|Map|Add (Variables|Progression|GetMainQuestsMap) "FinishedQuestGangMember" true)
            (Development|PrintText "Drug Dealer door opening...")))))))

(event Custom|DIsposedObjectUpdate
  (params (Capacity :type Integer))
  ;[0.15 0.15 0.15 0.5] UPDATING CLEANED & DISPOSED OBJECTS
  (if (< (Variables|Progression|GetDisposedObjects) (Variables|Progression|GetTotalObjectsToDispose))
    (bind _output_get (Variables|Progression|SetDisposedObjects (+ Capacity (Variables|Progression|GetDisposedObjects))))
    (Rendering|Components|TextRender|SetText (Variables|/Game/Blueprints/UI/WBP_ObjectiveList.WBP_ObjectiveList_C|GetObjectsDisposed (Variables|Default|GetObjective%20List)) (Utilities|Text|ToText(Integer) _output_get))
    (else
      (if (> (Variables|Progression|GetDisposedObjects) (Variables|Progression|GetTotalObjectsToDispose))
        (Variables|Progression|SetDisposedObjects (Variables|Progression|GetTotalObjectsToDispose)))
      (Utilities|Map|Add (Variables|Progression|GetMainQuestsMap) "FinishedDisposing" true))))

(event Custom|CleanedObjectUpdate
  ;[0.15 0.15 0.15 0.5] UPDATING CLEANED & DISPOSED OBJECTS
  (if (< (Variables|Progression|GetCleanedObjects) (Variables|Progression|GetTotalObjectsToClean))
    (bind _result (Math|Integer|IncrementInt (Variables|Progression|GetCleanedObjects))
      (:%20%20
        (Rendering|Components|TextRender|SetText (Variables|/Game/Blueprints/UI/WBP_ObjectiveList.WBP_ObjectiveList_C|GetObjectsCleaned (Variables|Default|GetObjective%20List)) (Utilities|Text|ToText(Integer) _result))))
    (else
      (if (> (Variables|Progression|GetCleanedObjects) (Variables|Progression|GetTotalObjectsToClean))
        (Variables|Progression|SetCleanedObjects (Variables|Progression|GetTotalObjectsToClean)))
      (Utilities|Map|Add (Variables|Progression|GetMainQuestsMap) "FinishedCleaning" true))))

(event Custom|InitializeUI
  ;[0.15 0.15 0.15 0.5] OBJECTIVE LIST UI
  (bind _returnvalue (UserInterface|CreateWidget "/Game/Blueprints/UI/WBP_ObjectiveList.WBP_ObjectiveList_C"))
  (UserInterface|Viewport|AddtoViewport _returnvalue 0)
  (Variables|Default|SetObjective%20List _returnvalue)
  (bind _returnvalue_2 (UserInterface|CreateWidget "/Game/Blueprints/UI/WBP_ScreenInputs.WBP_ScreenInputs_C"))
  (UserInterface|Viewport|AddtoViewport _returnvalue_2 0)
  (Variables|Default|SetScreen%20Input _returnvalue_2))

(event Custom|UpdateCleaningTasksUI
  (params (Index :type Integer))
  (Default|UpdateCleaningTasksUI (Variables|Default|GetObjective%20List) Index))

(event Custom|ToggleScreenInput
  (params (ScreenInputText :type Text) (IsActive%20 :type Boolean))
  (Default|ToggleScreenInput (Variables|Default|GetScreen%20Input) ScreenInputText IsActive%20))