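; BP_QuestManager is a quest manager that handles door-linked find-the-object quests and registers itself with BP_MainGameInstance on BeginPlay.
; UpdateQuest keeps a quest locked until enough objects are disposed of, then switches on the door's checkpoint.
; It activates the objective UI and messages the door to advance and spawn the object, reports progress, or toggles the completion checkbox.
; The door-opening call is unwired.
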(event Custom|UpdateQuest
  (params (Door :type Actor%20Object%20Reference) (Current%20Checkpoint :type Integer) (QuestActivationTreshold :type Integer))
  ;[0.15 0.15 0.15 0.5] CALLED BY GAMEINSTANCE, MANAGES IN-GAME QUEST EVENTS
  (bind _asbp_main_game_instance (Utilities|Casting|CastToBP_MainGameInstance (Game|GetGameInstance)))
  (if (< (Variables|/Game/Blueprints/Singletons/BP_MainGameInstance.BP_MainGameInstance_C|GetDisposedObjects _asbp_main_game_instance) QuestActivationTreshold)
    (Development|PrintString "Quest locked: clean some more before initiating")
    (else
      (Variables|Default|SetDoor Door)
      (Variables|Default|SetCurrent%20Checkpoint Current%20Checkpoint)
      (switch int (Variables|Default|GetCurrent%20Checkpoint)
        (:0
          (bind _asbp_main_game_instance_2 (Utilities|Casting|CastToBP_MainGameInstance (Game|GetGameInstance)))
          (Default|ActivateQuestUI (Variables|/Game/Blueprints/Singletons/BP_MainGameInstance.BP_MainGameInstance_C|GetObjective%20List _asbp_main_game_instance_2) (Variables|Default|GetDoor))
          (Class|BPIInterarct|IncrementCheckpoint(Message) (Variables|Default|GetDoor))
          (Class|BPIInterarct|SpawnQuestObject(Message) (Variables|Default|GetDoor)))
        (:1
          (Development|PrintString "Quest has started; go find the object"))
        (:2
          (bind _asbp_main_game_instance_3 (Utilities|Casting|CastToBP_MainGameInstance (Game|GetGameInstance)))
          (Development|PrintString "Quest has finished; door opening")
          (Default|ToggleQuestCheckBox (Variables|/Game/Blueprints/Singletons/BP_MainGameInstance.BP_MainGameInstance_C|GetObjective%20List _asbp_main_game_instance_3) (Variables|Default|GetDoor)))))))

(event EventBeginPlay
  ;[0.15 0.15 0.15 0.5] BEGIN PLAY
  (bind _asbp_main_game_instance (Utilities|Casting|CastToBP_MainGameInstance (Game|GetGameInstance)))
  (Variables|/Game/Blueprints/Singletons/BP_MainGameInstance.BP_MainGameInstance_C|SetQuest%20Manager%20Ref _asbp_main_game_instance self))

(event Collision|EventActorBeginOverlap
  (params (OtherActor :type Actor%20Object%20Reference)))

(event EventTick
  (params (DeltaSeconds :type Float%20%28single-precision%29)))

(fn ConstructionScript)