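; Tutorial script manager that guides the player through cleaning, trash burning and the cockroach introduction.
; On BeginPlay it possesses the cart, loads mop and swatter onto it, binds gameplay events and registers with the game instance.
; Those events and construction-script-positioned trigger boxes advance a checkpoint counter, whose switch runs each step: doors, item glows, ability unlocks, cockroach spawns.
; Focus triggers also lock the player and rotate the view toward points of interest.
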(event OnComponentBeginOverlap(FocusChangerToCollectGarbage)
  (params (OverlappedComponent :type Primitive%20Component%20Object%20Reference) (OtherActor :type Actor%20Object%20Reference) (OtherComp :type Primitive%20Component%20Object%20Reference) (OtherBodyIndex :type Integer) (bFromSweep :type Boolean) (SweepResult :type Hit%20Result%20Structure%20%28by%20ref%29))
  (bind _focuschangertocollectgarbage (Variables|Default|GetFocusChangerToCollectGarbage))
  ;[0.15 0.15 0.15 0.5] Va al sesto punto dello script
  (if (== OtherActor (Game|Player|GetPlayerPawn 0))
    (Utilities|IsValid _focuschangertocollectgarbage
      (:Is%20Valid
        (Collision|SetCollisionEnabled _focuschangertocollectgarbage "NoCollision")
        (CallFunction|ChangeFocus (Variables|FocusPoints|GetFocusPointCollectGarbage))
        (CallFunction|PlayScript))
      (:Is%20Not%20Valid
        (CallFunction|ChangeFocus (Variables|FocusPoints|GetFocusPointCollectGarbage))
        (CallFunction|PlayScript)))))

(event OnComponentBeginOverlap(FocusChangerToBurnTrash)
  (params (OverlappedComponent :type Primitive%20Component%20Object%20Reference) (OtherActor :type Actor%20Object%20Reference) (OtherComp :type Primitive%20Component%20Object%20Reference) (OtherBodyIndex :type Integer) (bFromSweep :type Boolean) (SweepResult :type Hit%20Result%20Structure%20%28by%20ref%29))
  (bind _focuschangertoburntrash (Variables|Default|GetFocusChangerToBurnTrash))
  ;[0.15 0.15 0.15 0.5] Va al settimo punto dello script
  (if (== OtherActor (Game|Player|GetPlayerPawn 0))
    (Utilities|IsValid _focuschangertoburntrash
      (:Is%20Valid
        (Collision|SetCollisionEnabled _focuschangertoburntrash "NoCollision")
        (CallFunction|ChangeFocus (Variables|FocusPoints|GetFocusPointToBurnTrash))
        (CallFunction|PlayScript))
      (:Is%20Not%20Valid
        (CallFunction|ChangeFocus (Variables|FocusPoints|GetFocusPointToBurnTrash))
        (CallFunction|PlayScript)))))

(event OnComponentBeginOverlap(TriggerZoneToCloseElevator)
  (params (OverlappedComponent :type Primitive%20Component%20Object%20Reference) (OtherActor :type Actor%20Object%20Reference) (OtherComp :type Primitive%20Component%20Object%20Reference) (OtherBodyIndex :type Integer) (bFromSweep :type Boolean) (SweepResult :type Hit%20Result%20Structure%20%28by%20ref%29))
  ;[0.15 0.15 0.15 0.5] va al secondo punto dello script
  (if (or (== OtherActor (Game|Player|GetPlayerPawn 0)) (== OtherActor (Variables|Default|GetMop)))
    (Utilities|IsValid (Variables|Default|GetTriggerZoneToCloseElevator)
      (:Is%20Valid
        (Collision|SetCollisionEnabled (Variables|Default|GetTriggerZoneToCloseElevator) "NoCollision")
        (CallFunction|PlayScript))
      (:Is%20Not%20Valid
        (CallFunction|PlayScript)))))

(event OnComponentBeginOverlap(FocusChangerToCleanseSins)
  (params (OverlappedComponent :type Primitive%20Component%20Object%20Reference) (OtherActor :type Actor%20Object%20Reference) (OtherComp :type Primitive%20Component%20Object%20Reference) (OtherBodyIndex :type Integer) (bFromSweep :type Boolean) (SweepResult :type Hit%20Result%20Structure%20%28by%20ref%29))
  ;[0.15 0.15 0.15 0.5] va al terzo punto dello script
  (if (== OtherActor (Game|Player|GetPlayerPawn 0))
    (Utilities|IsValid (Variables|Default|GetFocusChangerToCleanseSins)
      (:Is%20Valid
        (Collision|SetCollisionEnabled (Variables|Default|GetFocusChangerToCleanseSins) "NoCollision")
        (CallFunction|ChangeFocus (Variables|FocusPoints|GetFocusPointCleanseSins))
        (CallFunction|PlayScript))
      (:Is%20Not%20Valid
        (CallFunction|ChangeFocus (Variables|FocusPoints|GetFocusPointCleanseSins))
        (CallFunction|PlayScript)))))

(event OnComponentBeginOverlap(FocusChangerToCockroachDoor)
  (params (OverlappedComponent :type Primitive%20Component%20Object%20Reference) (OtherActor :type Actor%20Object%20Reference) (OtherComp :type Primitive%20Component%20Object%20Reference) (OtherBodyIndex :type Integer) (bFromSweep :type Boolean) (SweepResult :type Hit%20Result%20Structure%20%28by%20ref%29))
  (bind _focuschangertocockroachdoor (Variables|Default|GetFocusChangerToCockroachDoor))
  ;[0.15 0.15 0.15 0.5] Va all'ottavo punto dello script
  (if (== OtherActor (Game|Player|GetPlayerPawn 0))
    (Utilities|IsValid _focuschangertocockroachdoor
      (:Is%20Valid
        (Collision|SetCollisionEnabled _focuschangertocockroachdoor "NoCollision")
        (Variables|Default|SetCanBeEnabled false)
        (CallFunction|ChangeFocus (Variables|FocusPoints|GetFocusPointToCockroachDoor))
        (CallFunction|PlayScript))
      (:Is%20Not%20Valid
        (Variables|Default|SetCanBeEnabled false)
        (CallFunction|ChangeFocus)
        (CallFunction|PlayScript)))))

(event OnComponentBeginOverlap(TriggerZoneToEnlightSwatter)
  (params (OverlappedComponent :type Primitive%20Component%20Object%20Reference) (OtherActor :type Actor%20Object%20Reference) (OtherComp :type Primitive%20Component%20Object%20Reference) (OtherBodyIndex :type Integer) (bFromSweep :type Boolean) (SweepResult :type Hit%20Result%20Structure%20%28by%20ref%29))
  (bind _triggerzonetoenlightswatter (Variables|Default|GetTriggerZoneToEnlightSwatter))
  ;[0.15 0.15 0.15 0.5] Va al nono punto
  (if (== OtherActor (Game|Player|GetPlayerPawn 0))
    (Utilities|IsValid _triggerzonetoenlightswatter
      (:Is%20Valid
        (Collision|SetCollisionEnabled _triggerzonetoenlightswatter "NoCollision")
        (CallFunction|PlayScript))
      (:Is%20Not%20Valid
        (CallFunction|PlayScript)))))

(event Custom|Play_Script
  (bind _cart (Variables|Default|GetCart))
  (bind _waterbucket (Variables|/Game/Blueprints/Objects/BP_Cart.BP_Cart_C|GetWaterBucket _cart))
  (bind _childactor (Variables|/Script/Engine.ChildActorComponent|GetChildActor _waterbucket))
  ;[0.15 0.15 0.15 0.5] Qui avviene la magia
  (bind _result (Math|Integer|IncrementInt (Variables|Default|GetCheckPointNumber))
    (:%20%20
      (switch int _result
        (:1
          ;[0.15 0.15 0.15 0.5] Apre le porte dell'ascensore
          (Utilities|FlowControl|Delay 4.0)
          (Default|OpenElevatorDoorSX (Variables|Default|GetElevatorDoor_SX))
          (Default|OpenElevatorDoorDX (Variables|Default|GetElevatorDoor_DX))
          (Development|PrintString (Utilities|String|ToString(Integer) (Variables|Default|GetCheckPointNumber))))
        (:2
          ;[0.15 0.15 0.15 0.5] Chiude le porte dell'ascensore
          (Default|CloseElevatorDoorSX (Variables|Default|GetElevatorDoor_SX))
          (Default|CloseElevatorDoorDX (Variables|Default|GetElevatorDoor_DX))
          (Development|PrintString (Utilities|String|ToString(Integer) (Variables|Default|GetCheckPointNumber))))
        (:3
          ;[0.15 0.15 0.15 0.5] Illumina il mop per far capire al player che lo deve prendere
          (Class|BPICleaningTool|Glow(Message) (Variables|Default|GetMop))
          (Class|BPICleaningTool|SetCanbePicked(Message) (Variables|Default|GetMop))
          (Development|PrintString (Utilities|String|ToString(Integer) (Variables|Default|GetCheckPointNumber))))
        (:4
          ;[0.15 0.15 0.15 0.5] Gira la visuale verso la porta che si apre leggermente
          (CallFunction|ChangeFocus (Variables|FocusPoints|GetFocusPointFirstRoomToClean))
          (Default|DoorSlightlyOpensforTutorial (Variables|Default|GetDoorFirstRoomToClean))
          (Development|PrintString (Utilities|String|ToString(Integer) (Variables|Default|GetCheckPointNumber))))
        (:5
          ;[0.15 0.15 0.15 0.5] Illumina il water bucket per far capire al giocatore che deve lavare il mocio
          (Class|BPICleaningTool|Glow(Message) _childactor)
          (Class|BPICleaningTool|SetCanWashMop(Message) _childactor)
          (Variables|Default|SetCanGlow false)
          (Development|PrintString (Utilities|String|ToString(Integer) (Variables|Default|GetCheckPointNumber))))
        (:6
          ;[0.15 0.15 0.15 0.5] Illumina l'immondizia per far capire al player che deve buttarla
          (Class|BPICleaningTool|Glow(Message) (Variables|Default|GetTrash))
          (Default|CallOnTrashPickable)
          (Development|PrintString (Utilities|String|ToString(Integer) (Variables|Default|GetCheckPointNumber))))
        (:7
          ;[0.15 0.15 0.15 0.5] Illumina l'inceneritore per far capire al player di doverlo usare
          (Class|BPICleaningTool|Glow(Message) (Variables|Default|GetIncinerator))
          (Class|BPIPlayer|SetCanTakeTrashBag(Message) (Variables|Default|GetPlayer))
          (Variables|Default|SetIsFirstTimeTheTrashBagIsFull false)
          (Development|PrintString (Utilities|String|ToString(Integer) (Variables|Default|GetCheckPointNumber))))
        (:8
          ;[0.15 0.15 0.15 0.5] Apre la porta con gli scarafaggi così il player capisce che lì dentro li dovrà ammazzare
          (Default|DoorSlightlyOpensforTutorial (Variables|Default|GetCockroachDoor))
          (Utilities|FlowControl|Delay 3.0)
          (bind _returnvalue (Game|SpawnActorfromClass "/Game/Blueprints/AI/BP_NotInteractableCockroach.BP_NotInteractableCockroach_C" (Math|Transform|MakeTransform (Transformation|GetActorLocation (Variables|Default|GetCockroachSpawnPoint)) "0, 0, 0" "1.000000,1.000000,1.000000") "AlwaysSpawn" "MultiplyWithRoot" 0 0))
          (Default|CockroachGoOutOftheRoom _returnvalue (Variables|Default|GetCockroachTargetPoint1))
          (bind _returnvalue_2 (Game|SpawnActorfromClass "/Game/Blueprints/AI/BP_NotInteractableCockroach.BP_NotInteractableCockroach_C" (Math|Transform|MakeTransform (Transformation|GetActorLocation (Variables|Default|GetCockroachSpawnPoint)) "0, 0, 0" "1.000000,1.000000,1.000000") "AlwaysSpawn" "MultiplyWithRoot" 0 0))
          (Default|CockroachGoOutOftheRoom _returnvalue_2 (Variables|Default|GetCockroachTargetPoint2))
          (bind _returnvalue_3 (Game|SpawnActorfromClass "/Game/Blueprints/AI/BP_NotInteractableCockroach.BP_NotInteractableCockroach_C" (Math|Transform|MakeTransform (Transformation|GetActorLocation (Variables|Default|GetCockroachSpawnPoint)) "0, 0, 0" "1.000000,1.000000,1.000000") "AlwaysSpawn" "MultiplyWithRoot" 0 0))
          (Default|CockroachGoOutOftheRoom _returnvalue_3 (Variables|Default|GetCockroachTargetPoint3))
          (Development|PrintString (Utilities|String|ToString(Integer) (Variables|Default|GetCheckPointNumber)))
          (Utilities|FlowControl|Delay 1.0)
          (Collision|SetCollisionEnabled (Variables|Default|GetTriggerZoneToEnlightSwatter) "QueryOnly"))
        (:9
          ;[0.15 0.15 0.15 0.5] Illumina lo swatter così il player capisce che deve usarlo per uccidere gli scarafaggi
          (Class|BPICleaningTool|Glow(Message) (Variables|Default|GetSwatter))
          (Development|PrintString (Utilities|String|ToString(Integer) (Variables|Default|GetCheckPointNumber))))))))

(event Custom|Tutorial_Blood_Stain_Cleaned
  ;[1 1 1] Spawno come player ma mi attacco subito al cart. Serve per iniziare col cart attaccato e per passare i riferimenti che servono per il detach
  ;;[0.9946 0 1] Va al quarto punto dello script
  (CallFunction|PlayScript))

(event Custom|Enable_Collision
  ;[1 1 1] Spawno come player ma mi attacco subito al cart. Serve per iniziare col cart attaccato e per passare i riferimenti che servono per il detach
  ;;[0 0 1] Attiva la collisione del box dopo che il player ha usato l'inceneritore
  (if (Variables|Default|GetCanBeEnabled)
    (Collision|SetCollisionEnabled (Variables|Default|GetFocusChangerToCockroachDoor) "QueryOnly")))

(event Custom|OnMopFullyDirty_Event
  ;[1 1 1] Spawno come player ma mi attacco subito al cart. Serve per iniziare col cart attaccato e per passare i riferimenti che servono per il detach
  ;;[0 0.57 1] Va al quinto punto dello script
  (if (Variables|Default|GetCanGlow)
    (CallFunction|PlayScript)
    (Collision|SetCollisionEnabled (Variables|Default|GetFocusChangerToCollectGarbage) "QueryOnly")))

(event EventBeginPlay
  ;[1 1 1] Spawno come player ma mi attacco subito al cart. Serve per iniziare col cart attaccato e per passare i riferimenti che servono per il detach
  (bind _output_get (Variables|Default|SetPlayer (Game|Player|GetPlayerPawn 0)))
  (Utilities|IsValid _output_get
    (:Is%20Valid
      (Default|SetCanMove (Variables|Default|GetCart) true)
      (Default|GetOriginalPlayer (Variables|Default|GetCart) (Variables|Default|GetPlayer))
      (bind _playercollider (Class|BPIPlayer|GetCapsuleComponent(Message) (Variables|Default|GetPlayer)))
      (Collision|SetCollisionResponsetoChannel _playercollider "ECC_Pawn" "ECR_Ignore")
      (Default|DisableBinCollision (Variables|Default|GetCart))
      (Pawn|Possess (Game|GetPlayerController 0) (Variables|Default|GetCart))
      (Class|BPICart|PutObjectonCart(Message) (Variables|Default|GetCart) (Variables|Default|GetMop))
      (Class|BPICart|PutObjectonCart(Message) (Variables|Default|GetCart) (Variables|Default|GetSwatter))
      ;;[0.9946 0 1] Va al quarto punto dello script
      (EventDispatchers|AssignOnObjectCleaned (Variables|Default|GetFirstBloodStainToClean) (delegate Custom|Tutorial_Blood_Stain_Cleaned))
      ;;[0 0.57 1] Va al quinto punto dello script
      (EventDispatchers|AssignOnMopFullyDirty (Variables|/Game/Blueprints/Objects/Tools/BP_CleaningTool.BP_CleaningTool_C|GetBP_CleaningComp (Variables|Default|GetMop)) (delegate Custom|OnMopFullyDirty_Event))
      (Collision|SetCollisionEnabled (Variables|Default|GetFocusChangerToCockroachDoor) "NoCollision")
      ;;[0 0 1] Attiva la collisione del box dopo che il player ha usato l'inceneritore
      (EventDispatchers|BindEventtoOnTrashBurnt (Variables|Default|GetIncinerator) (delegate Custom|Enable_Collision))
      (Class|BPICart|SetObjectstoIgnorewithTrace(Message) (Variables|Default|GetCart) (Variables|Default|GetSwatter))
      (Collision|SetCollisionEnabled (Variables|Default|GetTriggerZoneToEnlightSwatter) "NoCollision")
      (Collision|SetCollisionEnabled (Variables|Default|GetFocusChangerToCollectGarbage) "NoCollision")
      (Collision|SetCollisionEnabled (Variables|Default|GetFocusChangerToBurnTrash) "NoCollision")
      (bind _asbp_main_game_instance (Utilities|Casting|CastToBP_MainGameInstance (Game|GetGameInstance)))
      (Variables|/Game/Blueprints/Singletons/BP_MainGameInstance.BP_MainGameInstance_C|SetScriptManager _asbp_main_game_instance self))))

(fn ConstructionScript
  (Transformation|SetRelativeTransform (Variables|Default|GetTriggerZoneToCloseElevator) (Variables|Transforms|GetTransformToCloseElevator) false false)
  (Transformation|SetRelativeTransform (Variables|Default|GetFocusChangerToCleanseSins) (Variables|Transforms|GetTransformFocusChangerToCleanseSins) false false)
  (Transformation|SetRelativeTransform (Variables|Default|GetFocusChangerToCollectGarbage) (Variables|Transforms|GetTransformToCollectGarbage) false false)
  (Transformation|SetRelativeTransform (Variables|Default|GetFocusChangerToBurnTrash) (Variables|Transforms|GetTransformToBurnTrash) false false)
  (Transformation|SetRelativeTransform (Variables|Default|GetFocusChangerToCockroachDoor) (Variables|Transforms|GetTransformToCockroachDoor) false false)
  (Transformation|SetRelativeTransform (Variables|Default|GetTriggerZoneToEnlightSwatter) (Variables|Transforms|GetTransformToEnlightSwatter) false false))

(fn ChangeFocus
  (params (FocusPoint :type Actor%20Object%20Reference))
  (LocalVariables|SetFocusObject FocusPoint)
  (Class|BPIPlayer|LockMovement(Message) (Game|Player|GetPlayerPawn 0))
  (Class|BPIPlayer|LockVision(Message) (Game|Player|GetPlayerPawn 0))
  (Class|BPIPlayer|RotatetoObject(Message) (Game|Player|GetPlayerPawn 0) (LocalVariables|GetFocusObject))
  (Collision|SetCollisionEnabled (Variables|Default|GetFocusChangerToCleanseSins) "NoCollision"))